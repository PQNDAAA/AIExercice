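; Base actor for a resource whose mesh and random starting quantity come from an item data table row in the construction script.
; Pressing the mesh sets a "selected" material parameter and shows a resource information widget; releasing clears both.
; DestroyResource hides the actor by teleporting it far away at zero scale rather than destroying it.
; Optional regeneration uses a timer to restore the saved transform and refill the inventory from ItemQuantity.
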(event OnReleased(StaticMesh)
  (params (TouchedComponent :type Primitive%20Component%20Object%20Reference) (ButtonReleased :type Key%20Structure))
  (Rendering|Material|SetScalarParameterValueonMaterials (Variables|Default|GetStaticMesh) "selected" 0.0)
  (Widget|RemovefromParent (Variables|Default|GetResourceInfo_Reference)))

(event OnClicked(StaticMesh)
  (params (TouchedComponent :type Primitive%20Component%20Object%20Reference) (ButtonPressed :type Key%20Structure))
  (Rendering|Material|SetScalarParameterValueonMaterials (Variables|Default|GetStaticMesh) "selected" 1.0)
  (bind _returnvalue (UserInterface|CreateWidget "/Game/Tools/ResourceTool/Widgets/WBP_ResourceInformation.WBP_ResourceInformation_C" 0 self))
  (bind _output_get (Variables|Default|SetResourceInfo_Reference _returnvalue))
  (UserInterface|Viewport|AddtoViewport _output_get 0))

(event Custom|TimerResourceRegeneration
  (params (ResourceRegenerationTime :type Float%20%28double-precision%29))
  ;[1 1 1] Start the timer
  (Utilities|Time|SetTimerbyFunctionName 0 "ResourceRegeneration" ResourceRegenerationTime))

(event EventBeginPlay
  (Variables|/Script/Engine.PlayerController|SetbEnableClickEvents (Game|GetPlayerController 0) true))

(event Collision|EventActorBeginOverlap
  (params (OtherActor :type Actor%20Object%20Reference)))

(event EventTick
  (params (DeltaSeconds :type Float%20%28single-precision%29)))

(fn ConstructionScript
  (bind _item (Variables|Default|GetItem))
  (bind (_datatable _rowname) (Utilities|Struct|BreakDataTableRowHandle _item))
  (bind _returnvalue (Utilities|GetDataTableRow _datatable _rowname)
    (:then
      (Variables|Default|SetS_Item _returnvalue)
      (Components|StaticMesh|SetStaticMesh (Variables|Default|GetStaticMesh) (.StaticMesh (Utilities|Struct|BreakS_Resources (Variables|Default|GetS_Item))))
      (Variables|Default|SetresourceInventory (Math|Random|RandomIntegerinRange (.QuantityMIN (Utilities|Struct|BreakS_Resources (Variables|Default|GetS_Item))) (.QuantityMAX (Utilities|Struct|BreakS_Resources (Variables|Default|GetS_Item))))))))

(fn ResourceRegeneration
  ;[1 1 1] Respawn the resource at the same transform with resources
  (Transformation|SetActorTransform (Variables|Default|GetOld%20Transform) false true)
  (Variables|Default|SetresourceInventory (.ItemQuantity (Utilities|Struct|BreakS_Resources (Variables|Default|GetS_Item)))))

(fn DestroyResource
  (params (Regeneration? :type Boolean))
  (Variables|Default|SetOld%20Transform (Transformation|GetActorTransform))
  (Transformation|SetActorTransform (Math|Transform|MakeTransform "2000000.000000,2000000.000000,2000000.000000" "0, 0, 0" "0.000000,0.000000,0.000000") false true)
  (if Regeneration?
    (CallFunction|TimerResourceRegeneration (Variables|/Game/Tools/MapEditorTool/BP/BP_BlockGenerated.BP_BlockGenerated_C|GetresourceRegenerationTime (CallFunction|GetMap)))
    (return true)
    (else
      (return true))))

(fn CheckResourceQuantity
  (if (!= (Variables|Default|GetresourceInventory) 0)
    (return false)
    (else
      (return true))))