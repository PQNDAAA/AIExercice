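; Procedural block-map generator for the map editor, rebuilt in the construction script from size, seed and frequency.
; FastNoise simplex heights drive a grid of instanced ground blocks, passing elevation and sand/rock thresholds to the material as custom data.
; Low cells get water instances; density rolls spawn trees (height-limited) and rocks as child actors from categorized classes.
; Ore placement only prints debug indices; a helper adjusts ground block height for buildings.
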(event Custom|CustomEvent_0)

(event EventBeginPlay)

(fn ConstructionScript
  (Utilities|Array|Clear (Variables|Default|GetIndexResources))
  (Utilities|Array|Clear (Variables|Default|GetIndexRocks))
  (GenerateMap|GenerateMap (Variables|MapConfiguration|GetSize) (Variables|MapConfiguration|GetSeed) (Variables|MapConfiguration|GetFrequency)))

(fn GenerateMap
  (params (Size :type Integer) (Seed :type Integer) (Frequency :type Float%20%28double-precision%29))
  (bind _loc (CallFunction|CalculateLocation))
  (bind _ground (Variables|Default|GetGround))
  (bind _returnvalue (Math|Vector|MakeVector (.x _loc) (.y _loc) (.z _loc)))
  ;[1 1 1] Setup Landscape
  (bind _returnvalue_2 (Game|ConstructObjectfromClass "/Script/FastNoiseGenerator.FastNoiseWrapper"))
  (bind _output_get (Variables|GenerateMap|SetFastNoiseWrapper _returnvalue_2))
  (Class|FastNoiseWrapper|SetupFastNoise _output_get "SimplexFractal" Seed Frequency "Quintic" "FBM" 2 2.0 0.5 0.45 "Natural" "CellValue")
  (CallFunction|SetColorMap)
  (for _index (range 0 Size)
    (Variables|GenerateMap|Setx (Math|Conversions|ToFloat(Integer) (- _index 1)))
    (for _index_2 (range 0 Size)
      (Variables|GenerateMap|Sety (Math|Conversions|ToFloat(Integer) (- _index_2 1)))
      (Variables|Default|SetElevation (.z _loc))
      (Variables|GenerateMap|SetGridVector _returnvalue)
      (CallFunction|GenerateGround (Variables|Default|GetGround) _returnvalue)
      ;[1 1 1] Set Custom Data value for the procedural material
      (Components|InstancedStaticMesh|SetCustomDataValue _ground (Variables|Default|GetIndex) 0 (Variables|Default|GetElevation) false)
      (Components|InstancedStaticMesh|SetCustomDataValue _ground (Variables|Default|GetIndex) 1 (Variables|MapConfiguration|GetSandHeight) false)
      (Components|InstancedStaticMesh|SetCustomDataValue _ground (Variables|Default|GetIndex) 2 (Variables|MapConfiguration|GetRockHeight) false)
      (bind _returnvalue_3 (Utilities|Array|Add (Variables|GenerateMap|GetGridCell) (Variables|GenerateMap|GetGridVector)))
      (CallFunction|GenerateWater)
      (CallFunction|GenerateEnvironement _returnvalue_3)
      (CallFunction|AddRockCell (Variables|GenerateMap|GetGridVector))
      (CallFunction|AddOres 0.0))))

(fn AddTrees
  (params (GridIndex%20 :type Integer) (TreeDensity :type Float%20%28double-precision%29) (HeightLimitRock :type Float%20%28double-precision%29) (HeightLimitByWater :type Boolean) (HeightLimitBySand :type Boolean))
  (bind _returnvalue (Math|Random|RandomFloatinRange 1.5 2.4))
  (bind _actorscategories (Variables|Default|GetActorsCategories))
  (bind _gridcell (Variables|GenerateMap|GetGridCell))
  (bind _output (Utilities|Array|Get(acopy) _gridcell GridIndex%20))
  (if (<= (Math|Random|RandomIntegerinRange 0 100) (* TreeDensity 1e+02))
    (if HeightLimitByWater
      (if (and (> (.z _output) (Variables|MapConfiguration|GetWaterHeight)) (< (.z _output) HeightLimitRock))
        (bind _returnvalue_2 (AddComponent|AddChildActorComponent false (Math|Transform|MakeTransform (Math|Vector|MakeVector (Math|Random|RandomFloatinRange (.x _output) (+ (.x _output) 1e+02)) (.y _output) (+ (.z _output) (* (Variables|MapConfiguration|GetBlockThickness) 1e+02))) (Math|Rotator|MakeRotator 0.0 0.0 (Math|Random|RandomFloatinRange 0.0 3.6e+02)) (Math|Vector|MakeVector _returnvalue _returnvalue _returnvalue)) :!label _label))
        (bind _keys (Utilities|Map|Keys _actorscategories))
        (for _array_element _keys
          (if (and (Utilities|Enum|Equal(Enum) (.Value (Utilities|Map|Find _actorscategories _array_element)) "NewEnumerator2") (!= _array_element 0))
            (Utilities|Array|AddUnique (Variables|Default|GetPlantsActors) _array_element)
            (ChildActorComponent|SetChildActorClass _returnvalue_2 (.OutItem (Utilities|Array|Random (Variables|Default|GetPlantsActors))))
            (Utilities|Array|AddUnique (Variables|Default|GetIndexResources) _returnvalue_2))))
      (elif HeightLimitBySand
        (if (and (> (.z _output) (Variables|MapConfiguration|GetSandHeight)) (< (.z _output) HeightLimitRock))
          (goto _label))
        (elif (< (.z _output) HeightLimitRock)
          (goto _label))))))

(fn AddEnvironments)

(fn AddRocks
  (params (GridIndex :type Integer) (RockDensity :type Float%20%28double-precision%29))
  (bind _returnvalue (Math|Random|RandomFloatinRange 0.2 0.65))
  (bind _actorscategories (Variables|Default|GetActorsCategories))
  (bind _gridcell (Variables|GenerateMap|GetGridCell))
  (bind _output (Utilities|Array|Get(acopy) _gridcell GridIndex))
  (if (<= (Math|Random|RandomIntegerinRange 0 100) (* RockDensity 1e+02))
    (bind _returnvalue_2 (AddComponent|AddChildActorComponent false (Math|Transform|MakeTransform (Math|Vector|MakeVector (Math|Random|RandomFloatinRange (.x _output) (+ (.x _output) 5e+01)) (Math|Random|RandomFloatinRange (.y _output) (+ (.y _output) 5e+01)) (+ (.z _output) (* (Variables|MapConfiguration|GetBlockThickness) 1e+02))) (Math|Rotator|MakeRotator 0.0 0.0 (Math|Random|RandomFloatinRange 0.0 3.6e+02)) (Math|Vector|MakeVector _returnvalue _returnvalue _returnvalue))))
    (bind _keys (Utilities|Map|Keys _actorscategories))
    (for _array_element _keys
      (if (Utilities|Enum|Equal(Enum) (.Value (Utilities|Map|Find _actorscategories _array_element)) "NewEnumerator1")
        (Utilities|Array|AddUnique (Variables|Default|GetRockActors) _array_element)
        (ChildActorComponent|SetChildActorClass _returnvalue_2 (.OutItem (Utilities|Array|Random (Variables|Default|GetRockActors))))
        (Utilities|Array|AddUnique (Variables|Default|GetIndexResources) _returnvalue_2)))))

(fn AddWater
  (bind _gridvector (Variables|GenerateMap|GetGridVector))
  (bind (_x _y) (Math|Vector|BreakVector _gridvector))
  (if (and (Variables|MapConfiguration|GetGeneratedWater?) (<= (Variables|Default|GetElevation) (Variables|MapConfiguration|GetWaterHeight)))
    (Components|InstancedStaticMesh|AddInstance (Variables|Default|GetWater) (Math|Transform|MakeTransform (Math|Vector|MakeVector _x _y (Variables|MapConfiguration|GetWaterHeight)) "0, 0, 0" "1.000000,1.000000,0.000000") false)))

(fn UpdateInstanceTransformPlaceBuilding
  (params (InstanceIndex :type Integer) (ActorZ :type Float%20%28double-precision%29))
  (bind _ground (Variables|Default|GetGround))
  (bind _outinstancetransform (Components|InstancedStaticMesh|GetInstanceTransform _ground InstanceIndex false))
  (Components|InstancedStaticMesh|UpdateInstanceTransform _ground InstanceIndex (Math|Transform|MakeTransform (Math|Vector|MakeVector (.x (.location _outinstancetransform)) (.y (.location _outinstancetransform)) (- ActorZ 1e+02)) (.rotation _outinstancetransform) (.scale _outinstancetransform)) false false true))

(fn AddOres
  (params (Height :type Float%20%28double-precision%29) (GridIndex :type Integer))
  (bind _actorscategories (Variables|Default|GetActorsCategories))
  (bind _oresactors (Variables|Default|GetOresActors))
  (bind _currentindex (LocalVariables|GetcurrentIndex))
  (bind _keys (Utilities|Map|Keys _actorscategories))
  (for _array_element _keys
    (if (Utilities|Enum|Equal(Enum) (.Value (Utilities|Map|Find _actorscategories _array_element)) "NewEnumerator4")
      (Utilities|Array|AddUnique (Variables|Default|GetOresActors) _array_element)))
  (bind (_array_element_2 _array_index) (Utilities|Array|ForEachLoopwithBreak _oresactors :!label _label)
    (:LoopBody
      (if (Utilities|Array|IsValidIndex _oresactors _currentindex)
        (if (== _array_index _currentindex)
          (bind _asbp_resource_base (Utilities|Casting|CastToBP_ResourceBaseClass _array_element_2))
          (bind _returnvalue (Utilities|GetDataTableRow (.DataTable (Utilities|Struct|BreakDataTableRowHandle (.Item (Utilities|GetClassDefaults _asbp_resource_base)))) (.RowName (Utilities|Struct|BreakDataTableRowHandle (.Item (Utilities|GetClassDefaults _asbp_resource_base)))))
            (:then
              (for _index (range 0 (- (Math|Float|Truncate (* (.Density (Utilities|Struct|BreakS_Resources _returnvalue)) (Utilities|Array|Length (Variables|Default|GetRockCell)))) 1))
                (Development|PrintString (Utilities|String|ToString(Integer) _index))
                (goto _label Break)))))
        (else
          (goto _label Break))))))

(fn GenerateEnvironement
  (params (Index :type Integer))
  (GenerateMap|AddTrees Index (Variables|MapConfiguration|GetTreeDensity) (Variables|MapConfiguration|GetRockHeight) (Variables|MapConfiguration|GetTreeHeightLimitByWater) (Variables|MapConfiguration|GetTreeHeightLimitbySand))
  (CallFunction|AddOres (Variables|MapConfiguration|GetRockHeight) Index)
  (GenerateMap|AddRocks Index (Variables|MapConfiguration|GetRockDensity)))

(fn GenerateWater
  (GenerateMap|AddWater)
  (bind _returnvalue (Rendering|Material|CreateDynamicMaterialInstance (Variables|Default|GetWater) 0 "/Game/Landscape/Materials/Water.Water" "None" :!class /Script/Engine.PrimitiveComponent))
  ;[1 1 1] Water Color
  (Rendering|Material|SetVectorParameterValue _returnvalue "Water" (Variables|ColorConfiguration|GetWaterColor) :!class /Script/Engine.MaterialInstanceDynamic))

(fn GenerateGround
  (params (Target :type Instanced%20Static%20Mesh%20Component%20Object%20Reference) (loc :type Vector))
  (Components|StaticMesh|SetStaticMesh Target (Variables|Meshes|GetGroundMesh))
  (bind _returnvalue (Components|InstancedStaticMesh|AddInstance Target (Math|Transform|MakeTransform loc "0, 0, 0" "1.000000,1.000000,1.000000") false))
  (bind _output_get (Variables|Default|SetIndex _returnvalue))
  (Components|InstancedStaticMesh|UpdateInstanceTransform Target _output_get (Math|Transform|MakeTransform (.location (.OutInstanceTransform (Components|InstancedStaticMesh|GetInstanceTransform Target _output_get false))) (.rotation (.OutInstanceTransform (Components|InstancedStaticMesh|GetInstanceTransform Target _output_get false))) (Math|Vector|MakeVector 1.0 1.0 (Variables|MapConfiguration|GetBlockThickness))) false false false))

(fn SetColorMap
  (bind _returnvalue (Rendering|Material|CreateDynamicMaterialInstance (Variables|Default|GetGround) 0 "/Game/Landscape/Materials/Ground_Inst.Ground_Inst" "None" :!class /Script/Engine.PrimitiveComponent))
  ;[1 1 1] Material's Color
  (Rendering|Material|SetVectorParameterValue _returnvalue "Sand" (Variables|ColorConfiguration|GetSandColor) :!class /Script/Engine.MaterialInstanceDynamic)
  (Rendering|Material|SetVectorParameterValue _returnvalue "Landscape" (Variables|ColorConfiguration|GetLandscape1) :!class /Script/Engine.MaterialInstanceDynamic)
  (Rendering|Material|SetVectorParameterValue _returnvalue "Landscape2" (Variables|ColorConfiguration|GetLandscape2) :!class /Script/Engine.MaterialInstanceDynamic))

(fn CalculateLocation
  (return (Math|Vector|MakeVector (* (Variables|GenerateMap|Getx) (Variables|GenerateMap|GetDistance)) (* (Variables|GenerateMap|Gety) (Variables|GenerateMap|GetDistance)) (* (Class|FastNoiseWrapper|GetNoise2D (Variables|GenerateMap|GetFastNoiseWrapper) (Variables|GenerateMap|Getx) (Variables|GenerateMap|Gety)) (Variables|MapConfiguration|GetMapHeight)))))

(fn AddRockCell
  (params (CurrentGridVector :type Vector))
  (if (>= (.z CurrentGridVector) (Variables|MapConfiguration|GetRockHeight))
    (Utilities|Array|AddUnique (Variables|Default|GetRockCell) (Math|Vector|MakeVector (.x CurrentGridVector) (.y CurrentGridVector) (.z CurrentGridVector)))))