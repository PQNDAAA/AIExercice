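; Town hall building that acts as a resource store, with each resource type capped at MaxResources.
; On BeginPlay it seeds ResourceMap from VirtualInventory via DT_Resources, and later additions clamp overflow, returning false only if already full.
; Recipe check and subtract functions map item classes to resource names through their class-default data table rows.
; The construction script places the supply Point just beyond the Box's X extent.
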(event EventBeginPlay
  (CallFunction|AddResourcesTownHallBeginning))

(event EventTick
  (params (DeltaSeconds :type Float%20%28single-precision%29)))

(fn ConstructionScript
  (bind _point (Variables|Default|GetPoint))
  (bind _relativelocation (Variables|/Script/Engine.SceneComponent|GetRelativeLocation _point))
  (|CallParentFunction)
  ;[1 1 1] Attach the supply point to the Box
  (Transformation|SetRelativeLocation _point (Math|Vector|MakeVector (+ (.x (Variables|/Script/Engine.BoxComponent|GetBoxExtent (Variables|Default|GetBox))) 4e+01) (.y _relativelocation) (.z _relativelocation)) false false))

(fn AddResourcesTownHallBeginning
  (bind _maxresources (Variables|Default|GetmaxResources))
  (bind _resourcemap (Variables|Default|GetResourceMap))
  (bind _keys (Utilities|Map|Keys (Variables|Default|GetvirtualInventory)))
  (for _array_element _keys
    (bind _returnvalue (Utilities|GetDataTableRow "/Game/Tools/ResourceTool/Datatable/DT_Resources.DT_Resources" (Utilities|String|StringToName _array_element))
      (:then
        ;[1 1 1] Calculate the excess quantity if the quantity is higher or not
        (LocalVariables|SetResourceType (Utilities|String|ToString(Name) (.Name (Utilities|Struct|BreakS_Resources _returnvalue))))
        (if (< (.Value (Utilities|Map|Find (Variables|Default|GetvirtualInventory) (LocalVariables|GetResourceType))) _maxresources)
          (Utilities|Map|Add _resourcemap (LocalVariables|GetResourceType) (.Value (Utilities|Map|Find (Variables|Default|GetvirtualInventory) (LocalVariables|GetResourceType))))
          (else
            (bind _quantitytoadd (ExcessQuantity|CalculateExcessQuantity (.Value (Utilities|Map|Find (Variables|Default|GetvirtualInventory) (LocalVariables|GetResourceType))) _maxresources (.Value (Utilities|Map|Find (Variables|Default|GetvirtualInventory) (LocalVariables|GetResourceType)))))
            (Utilities|Map|Add _resourcemap (LocalVariables|GetResourceType) _quantitytoadd))))
      (:RowNotFound
        (Development|PrintString "Resource not found")))))

(fn SubstractResourcesTownHall
  (params (Recipe :type Map%20of%20BP%20Resource%20Base%20Class%20References%20to%20Integers))
  (bind _resourcemap (Variables|Default|GetResourceMap))
  (bind _keys (Utilities|Map|Keys Recipe))
  (for _array_element _keys
    (LocalVariables|SetRemainingQuantity (.Value (Utilities|Map|Find Recipe _array_element)))
    (bind _returnvalue (Utilities|GetDataTableRow (.DataTable (Utilities|Struct|BreakDataTableRowHandle (.Item (Utilities|GetClassDefaults _array_element)))) (.RowName (Utilities|Struct|BreakDataTableRowHandle (.Item (Utilities|GetClassDefaults _array_element)))))
      (:then
        (Utilities|Map|Add _resourcemap (Utilities|String|ToString(Name) (.Name (Utilities|Struct|BreakS_Resources _returnvalue))) (- (.Value (Utilities|Map|Find _resourcemap (Utilities|String|ToString(Name) (.Name (Utilities|Struct|BreakS_Resources _returnvalue))))) (LocalVariables|GetRemainingQuantity)))))))

(fn AddResourcesTownHall
  (params (ResourceType :type String) (quantityToAdd :type Integer))
  (bind _resourcemap (Variables|Default|GetResourceMap))
  (bind _maxresources (Variables|Default|GetmaxResources))
  (bind _resourcemap_2 (Variables|Default|GetResourceMap))
  ;[1 1 1] Setup local variables
  (LocalVariables|SetResourceToAdd ResourceType)
  (LocalVariables|SetRemainingQuantity quantityToAdd)
  (bind _returnvalue (Utilities|GetDataTableRow "/Game/Tools/ResourceTool/Datatable/DT_Resources.DT_Resources" (Utilities|String|StringToName (LocalVariables|GetResourceToAdd)))
    (:then
      (if (< (.Value (Utilities|Map|Find (Variables|Default|GetResourceMap) (Utilities|String|ToString(Name) (.Name (Utilities|Struct|BreakS_Resources _returnvalue))))) _maxresources)
        (if (.notExcess (ExcessQuantity|CheckExcessQuantity (.Value (Utilities|Map|Find (Variables|Default|GetResourceMap) (Utilities|String|ToString(Name) (.Name (Utilities|Struct|BreakS_Resources _returnvalue))))) _maxresources (LocalVariables|GetRemainingQuantity)))
          ;[1 1 1] Add
          (Utilities|Map|Add _resourcemap (LocalVariables|GetResourceToAdd) (+ (.Value (Utilities|Map|Find _resourcemap (LocalVariables|GetResourceToAdd))) (LocalVariables|GetRemainingQuantity)))
          (return true)
          (else
            ;[1 1 1] Calculate the excess quantity
            (bind _quantitytoadd (ExcessQuantity|CalculateExcessQuantity (LocalVariables|GetRemainingQuantity) (Variables|Default|GetmaxResources) (.excessQuantity (ExcessQuantity|CheckExcessQuantity (.Value (Utilities|Map|Find (Variables|Default|GetResourceMap) (Utilities|String|ToString(Name) (.Name (Utilities|Struct|BreakS_Resources _returnvalue))))) _maxresources (LocalVariables|GetRemainingQuantity)))))
            (Utilities|Map|Add _resourcemap_2 (LocalVariables|GetResourceToAdd) (+ (.Value (Utilities|Map|Find _resourcemap_2 (LocalVariables|GetResourceToAdd))) _quantitytoadd))
            (return true)))
        (else
          (return false))))))

(fn CheckExcessQuantity
  (params (currentResourceQuantityTownHall :type Integer) (maxResources :type Integer) (remainingQuantity :type Integer))
  (bind _returnvalue (+ currentResourceQuantityTownHall remainingQuantity))
  (if (<= _returnvalue maxResources)
    (return true 0)
    (else
      (return false _returnvalue))))

(fn CalculateExcessQuantity
  (params (remainingQuantity :type Integer) (maxResources :type Integer) (excessQuantity :type Integer))
  (return (- remainingQuantity (- excessQuantity maxResources))))

(fn CheckRecipeQuantityTownHall
  (params (Recipe :type Map%20of%20BP%20Resource%20Base%20Class%20References%20to%20Integers))
  (LocalVariables|SetquantitesAreCorrect? true)
  (bind _output_get (LocalVariables|SetrecipeReference Recipe))
  (bind _keys (Utilities|Map|Keys _output_get))
  (if (Utilities|Array|IsEmpty _keys)
    (bind _output_get_2 (LocalVariables|SetquantitesAreCorrect? false))
    (return _output_get_2)
    (else
      (bind _array_element (Utilities|Array|ForEachLoopwithBreak _keys :!label _label)
        (:LoopBody
          (bind _returnvalue (Utilities|GetDataTableRow (.DataTable (Utilities|Struct|BreakDataTableRowHandle (.Item (Utilities|GetClassDefaults _array_element)))) (.RowName (Utilities|Struct|BreakDataTableRowHandle (.Item (Utilities|GetClassDefaults _array_element)))))
            (:then
              (if (not (and (.ReturnValue (Utilities|Map|Find (Variables|Default|GetResourceMap) (Utilities|String|ToString(Name) (.Name (Utilities|Struct|BreakS_Resources _returnvalue))))) (>= (.Value (Utilities|Map|Find (Variables|Default|GetResourceMap) (Utilities|String|ToString(Name) (.Name (Utilities|Struct|BreakS_Resources _returnvalue))))) (.Value (Utilities|Map|Find (LocalVariables|GetrecipeReference) _array_element)))))
                (LocalVariables|SetquantitesAreCorrect? false)
                (goto _label Break)))))
        (:Completed
          (return (LocalVariables|GetquantitesAreCorrect?)))))))