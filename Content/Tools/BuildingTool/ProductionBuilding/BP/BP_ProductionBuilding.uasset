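; BP_ProductionBuilding is a building that passively produces a configured resource for the Town Hall.
; From BeginPlay, a self-looping Delay on RewardDelay repeatedly calls AddResources with a fixed quantity.
; AddResources finds the Town Hall, looks up the resource in DT_Resources and deposits it.
; A successful deposit grants the player pawn's LevellingComponent the row's reward EXP, multiplied by the quantity.
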(event EventBeginPlay
  (|CallParentFunction)
  ;[1 1 1] The production System
  (Utilities|FlowControl|Delay (Variables|Default|GetrewardDelay) :!label _label)
  (CallFunction|AddResources 5 (Variables|Default|GetresourceToProduce))
  (goto _label))

(event Collision|EventActorBeginOverlap
  (params (OtherActor :type Actor%20Object%20Reference))
  (|CallParentFunction OtherActor) ; This node is disabled and will not be called.\nDrag off pins to build functionality.
)

(event EventTick
  (params (DeltaSeconds :type Float%20%28single-precision%29))
  (|CallParentFunction DeltaSeconds) ; This node is disabled and will not be called.\nDrag off pins to build functionality.
)

(fn ConstructionScript
  (|CallParentFunction))

(fn AddResources
  (params (Quantity :type Integer) (RowName :type Name))
  (bind (_find_ _townhallreference) (CallFunction|FindTownHall))
  (if _find_
    (LocalVariables|SetremainingQuantity Quantity)
    (LocalVariables|SetTownHallReference _townhallreference)
    (bind _returnvalue (Utilities|GetDataTableRow "/Game/Tools/ResourceTool/Datatable/DT_Resources.DT_Resources" RowName)
      (:then
        ;[1 1 1] Update Quantity TownHall
        (bind _isadded (Default|AddResourcesTownHall (LocalVariables|GetTownHallReference) (Utilities|String|ToString(Name) (.Name (Utilities|Struct|BreakS_Resources _returnvalue))) (LocalVariables|GetremainingQuantity)))
        (if _isadded
          ;[1 1 1] Add Exp each time
          (bind _asbp_character_pawn (Utilities|Casting|CastToBP_CharacterPawn (Game|Player|GetPlayerPawn 0)))
          (Default|AddExp (Variables|/Game/Player/BP/BP_CharacterPawn.BP_CharacterPawn_C|GetLevellingComponent _asbp_character_pawn) (.RewardExp (Utilities|Struct|BreakS_Resources _returnvalue)) (LocalVariables|GetremainingQuantity)))))))