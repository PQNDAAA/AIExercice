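; Placeable building actor from the building tool that adjusts the map and clears resources within its footprint.
; The construction script aligns a box to the static mesh and sizes it from the placement area.
; When the box begins overlapping the map's instanced ground, it passes the hit instance and building Z to the map to lower that ground.
; A separate function gathers overlapping resource actors and calls their destroy function.
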(event OnComponentBeginOverlap(Box)
  (params (OverlappedComponent :type Primitive%20Component%20Object%20Reference) (OtherActor :type Actor%20Object%20Reference) (OtherComp :type Primitive%20Component%20Object%20Reference) (OtherBodyIndex :type Integer) (bFromSweep :type Boolean) (SweepResult :type Hit%20Result%20Structure%20%28by%20ref%29))
  (bind _returnvalue (CallFunction|GetMap))
  ;[1 1 1] Reduce the ground height when the building is placed
  (if (== OtherComp (Variables|/Game/Tools/MapEditorTool/BP/BP_BlockGenerated.BP_BlockGenerated_C|GetGround _returnvalue))
    (Default|UpdateInstanceTransformPlaceBuilding _returnvalue (.HitItem (Collision|BreakHitResult SweepResult)) (.z (Transformation|GetActorLocation)))))

(event EventBeginPlay)

(event Collision|EventActorBeginOverlap
  (params (OtherActor :type Actor%20Object%20Reference)))

(event EventTick
  (params (DeltaSeconds :type Float%20%28single-precision%29)))

(fn ConstructionScript
  (bind _placementarea (Variables|Default|GetplacementArea))
  ;[1 1 1] Attach The box to the static Mesh
  (Transformation|SetRelativeLocation (Variables|Default|GetBox) (Variables|/Script/Engine.SceneComponent|GetRelativeLocation (Variables|Default|GetStaticMesh)) false false)
  ;[1 1 1] Setup the box thanks to the placement area
  (Components|Box|SetBoxExtent (Variables|Default|GetBox) (Math|Vector|MakeVector _placementarea _placementarea _placementarea) true))

(fn SetBoxLocation
  (params (Target :type Scene%20Component%20Object%20Reference))
  (Transformation|SetRelativeLocation (Variables|Default|GetBox) (Variables|/Script/Engine.SceneComponent|GetRelativeLocation Target) false false))

(fn DestroyResourceOverlapBuilding
  (for _array_element (Collision|GetOverlappingActors (Variables|Default|GetBox) "/Game/Tools/ResourceTool/BP/BP_ResourceBase.BP_ResourceBase_C" :!class /Script/Engine.PrimitiveComponent)
    (Utilities|Array|AddUnique (Variables|Default|GetresourceOverlapBuilding) _array_element))
  (for _array_element_2 (Variables|Default|GetresourceOverlapBuilding)
    (bind _asbp_resource_base (Utilities|Casting|CastToBP_ResourceBase _array_element_2))
    (Default|DestroyResource _asbp_resource_base false))
  (Utilities|Array|Clear (Variables|Default|GetresourceOverlapBuilding)))