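; BP_WorkBuildingBase is a base Blueprint for work buildings that employ villagers.
; Its construction script applies the configured static mesh and sizes a sphere search area from the SearchArea value.
; Helper functions add or remove current villagers and check for free capacity or a match with the building's target job.
; On BeginPlay it enables click events on the player controller.
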(event EventBeginPlay
  (Variables|/Script/Engine.PlayerController|SetbEnableClickEvents (Game|GetPlayerController 0) true))

(fn ConstructionScript
  (|CallParentFunction)
  (Components|StaticMesh|SetStaticMesh (Variables|Default|GetStaticMesh) (Variables|Default|GetStatic_Mesh_Reference))
  ;[1 1 1] Set the Search Area with the Sphere
  (Components|Sphere|SetSphereRadius (Variables|Default|GetSphereSearchArea) (Variables|Informations|GetsearchArea) true))

(fn AddPeople
  (params (value :type Integer))
  (Variables|Informations|SetcurrentVillagers (+ value (Variables|Informations|GetcurrentVillagers))))

(fn ReducePeople
  (params (value :type Integer))
  (Variables|Informations|SetcurrentVillagers (- (Variables|Informations|GetcurrentVillagers) value)))

(fn CheckCharacterCapacityWorkBuilding
  (if (< (Variables|Informations|GetcurrentVillagers) (Variables|Informations|GetvillagersMax))
    (return true)
    (else
      (return false))))

(fn CheckCharacterJobsWorkBuilding
  (params (Jobs :type Enum_Jobs%20Enum :default "NewEnumerator0"))
  (if (Utilities|Enum|Equal(Enum) (Variables|Informations|GetTargetJobs) Jobs)
    (return true)
    (else
      (return false))))