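; Villager character that autonomously finds a job at a matching work building, gathers resources and delivers them to the town hall.
; Recursive events with AIMoveTo loop through searching the building's area, collecting a unit, depositing and resting, wandering randomly when no work exists.
; Collecting grants player XP and destroys depleted resources.
; A parallel hunger timer eats town hall wheat when low and destroys the villager at zero.
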(event Custom|GoToBase
  (bind _resourceinventory (Variables|BasicStats|GetresourceInventory))
  ;[1 1 1] Go to base
  (Variables|Boolean|SetisGoingAtBase true)
  (AI|AIMoveTo self (Transformation|GetWorldLocation (Variables|/Game/Tools/BuildingTool/TownHallBuilding/BP/BP_TownHall.BP_TownHall_C|GetPoint (Variables|Default|GetTown%20Hall%20Reference))) 0 1e+02 false
    (:OnSuccess
      (bind _keys (Utilities|Map|Keys _resourceinventory))
      ;;[1 1 1] Add Resource in the town hall and clear the inventory
      (Default|AddResourcesTownHall (Variables|Default|GetTown%20Hall%20Reference) (Utilities|Array|Get(acopy) _keys) (.Value (Utilities|Map|Find _resourceinventory (Utilities|Array|Get(acopy) _keys))))
      (CharacterInventory|ClearCharacterInventory)
      ;;[1 1 1] Break
      (Utilities|FlowControl|Delay (Variables|BasicStats|GetDurationForBreak))
      (Variables|Boolean|SetisGoingAtBase false)
      (CallFunction|SearchWork))))

(event Custom|RandomLocationWithoutWorkBuilding
  ;[1 1 1] If the work building is destroyed then the character walks randomly without work building
  (AI|AIMoveTo self (.RandomLocation (AI|Navigation|GetRandomReachablePointinRadius (Transformation|GetActorLocation) 4e+02 0 0)) 0 5e+01 false
    (:OnSuccess
      _)
    (:OnFail
      _))
  (Utilities|FlowControl|Delay 1.0)
  (bind _isfound_ (CallFunction|SearchWorkBuilding))
  (if _isfound_
    (CallFunction|SearchWork)
    (else
      (CallFunction|RandomLocationWithoutWorkBuilding))))

(event Custom|GoToWork
  ;[1 1 1] Go to Work
  (Variables|Boolean|SetisGoingAtWork? true)
  (AI|AIMoveTo self (Variables|Vector|Getdestination) 0 3e+01 false
    (:then
      ;;[1 1 1] Check if the item to collect is always available
      (CallFunction|CheckItemQuantitytoCollect))
    (:OnSuccess
      ;;[1 1 1] Add Resource Player Inventory
      (bind _isempty_ (CharacterInventory|AddResourceCharacterInventory (Variables|Default|GetItemToCollect)))
      ;;[1 1 1] If the resource is empty then DESTROY IT
      (if _isempty_
        (bind _asbp_resource_base (Utilities|Casting|CastToBP_ResourceBase (Variables|Default|GetItemToCollect)))
        (Default|DestroyResource _asbp_resource_base true))
      (Variables|Boolean|SetisGoingAtWork? false)
      (CallFunction|GotoBase))))

(event Custom|RandomLocationWithoutWork
  ;[1 1 1] If no work then the character walks randomly around the search area
  (if (and (== (Variables|Boolean|GetisGoingAtWork?) false) (== (Variables|Boolean|GetisGoingAtBase) false))
    (AI|AIMoveTo self (.RandomLocation (AI|Navigation|GetRandomReachablePointinRadius (Transformation|GetActorLocation (Variables|Default|GetTargetWorkBuilding)) (/ (Variables|BasicStats|GetsearchArea) 2.0) 0 0)) 0 5e+01 false
      (:OnSuccess
        _)
      (:OnFail
        _))
    (Utilities|FlowControl|Delay 1.0)
    (CallFunction|SearchWork)
    (else
      (Utilities|FlowControl|Delay 0.2)
      (CallFunction|RandomLocationWithoutWork))))

(event Custom|HungerUpdate
  ;[1 1 1] Hunger Loop
  (if (<= (Variables|BasicStats|GetHunger) 0)
    (Default|ReducePeople (Variables|Default|GetTargetWorkBuilding) 1)
    (Actor|DestroyActor)
    (else
      (Utilities|FlowControl|Delay 2.0)
      (Hunger|RemoveHunger (Variables|BasicStats|GetHungerToRemove))
      (Hunger|CheckHunger (Variables|BasicStats|GetHunger%20Alert) (Variables|BasicStats|GetQuantity%20to%20Add%20Alert))
      (CallFunction|HungerUpdate))))

(event Custom|SearchWork
  ;[1 1 1] When the character search a place to work
  (Variables|Boolean|SetisGoingAtWork? false)
  (bind _found_ (CallFunction|FindResources (Variables|BasicStats|GetJobs)))
  (if _found_
    (CallFunction|GotoWork)
    (else
      (CallFunction|RandomLocationWithoutWork))))

(event Custom|CheckItemQuantityToCollect
  ;[1 1 1] Check when the character is going at work so after find resources
  (if (Variables|Boolean|GetisGoingAtWork?)
    ;[1 1 1] Check the quantity example -> if another character takes the last resource before, the character will go "Search Work"
    (bind _asbp_resource_base (Utilities|Casting|CastToBP_ResourceBase (Variables|Default|GetItemToCollect)))
    (bind _isempty_ (Default|CheckResourceQuantity _asbp_resource_base))
    (if _isempty_
      (CallFunction|SearchWork)
      (else
        (Utilities|FlowControl|Delay 0.2)
        (CallFunction|CheckItemQuantitytoCollect)))))

(event EventBeginPlay
  (Utilities|FlowControl|Delay 1.0)
  (bind (_find_ _townhallreference) (CallFunction|FindTownHall))
  (Variables|Default|SetTown%20Hall%20Reference _townhallreference)
  (if _find_
    (CallFunction|SetCharacterWidgetName (Variables|Default|GetWidget))
    (CallFunction|HungerUpdate)
    ;[1 1 1] Game Loop starts
    (bind _isfound_ (CallFunction|SearchWorkBuilding))
    (if _isfound_
      (CallFunction|SearchWork)
      (else
        (CallFunction|RandomLocationWithoutWorkBuilding)))
    (else
      (Actor|DestroyActor))))

(fn ConstructionScript
  (Variables|/Script/Engine.CharacterMovementComponent|SetMaxWalkSpeed (Variables|Character|GetCharacterMovement) (Variables|BasicStats|GetdefaultValueSpeed)))

(fn SearchWorkBuilding
  (LocalVariables|SethasFound? false)
  (bind _outactors (Actor|GetAllActorsOfClass "/Game/Tools/BuildingTool/WorkBuilding/BP/BP_WorkBuildingBase.BP_WorkBuildingBase_C"))
  (bind _array_element (Utilities|Array|ForEachLoopwithBreak _outactors)
    (:LoopBody
      (if (Math|Boolean|ANDBoolean (== (Utilities|Array|Get(acopy) (Variables|/Script/Engine.Actor|GetTags _array_element)) "Building") (Default|CheckCharacterJobsWorkBuilding _array_element (Variables|BasicStats|GetJobs)) (Default|CheckCharacterCapacityWorkBuilding _array_element))
        (LocalVariables|SethasFound? true)
        (bind _output_get (Variables|Default|SetTargetWorkBuilding _array_element))
        (Variables|BasicStats|SetsearchArea (Variables|/Game/Tools/BuildingTool/WorkBuilding/BP/BP_WorkBuildingBase.BP_WorkBuildingBase_C|GetsearchArea _output_get))
        (Default|AddPeople (Variables|Default|GetTargetWorkBuilding) 1)
        (return (LocalVariables|GethasFound?))))
    (:Completed
      (if (== (LocalVariables|GethasFound?) false)
        (return (LocalVariables|GethasFound?))))))

(fn SetCharacterWidgetName
  (params (Widget :type Widget%20Component%20Object%20Reference))
  (bind _aswbp_character_bar_name (Utilities|Casting|CastToWBP_CharacterBarName (UserInterface|GetUserWidgetObject Widget)))
  (Rendering|Components|TextRender|SetText (Variables|/Game/Tools/CharactersTool/Characters/Widgets/WBP_CharacterBarName.WBP_CharacterBarName_C|GetnameText _aswbp_character_bar_name) (Utilities|Text|ToText(String) (Utilities|String|ToString(Name) (Variables|BasicStats|GetName)))))

(fn AddResourceCharacterInventory
  (params (Item :type Actor%20Object%20Reference))
  (bind _asbp_resource_base (Utilities|Casting|CastToBP_ResourceBase Item))
  (Utilities|Map|Add (Variables|BasicStats|GetresourceInventory) (Utilities|String|ToString(Name) (.Name (Utilities|Struct|BreakS_Resources (Variables|/Game/Tools/ResourceTool/BP/BP_ResourceBase.BP_ResourceBase_C|GetS_Item _asbp_resource_base)))) 1)
  ;[1 1 1] Substract the resource in the target item
  (Variables|/Game/Tools/ResourceTool/BP/BP_ResourceBase.BP_ResourceBase_C|SetresourceInventory _asbp_resource_base (- (Variables|/Game/Tools/ResourceTool/BP/BP_ResourceBase.BP_ResourceBase_C|GetresourceInventory _asbp_resource_base) 1))
  (bind _asbp_character_pawn (Utilities|Casting|CastToBP_CharacterPawn (Game|Player|GetPlayerPawn 0)))
  (Default|AddExp (Variables|/Game/Player/BP/BP_CharacterPawn.BP_CharacterPawn_C|GetLevellingComponent _asbp_character_pawn) (.RewardExp (Utilities|Struct|BreakS_Resources (Variables|/Game/Tools/ResourceTool/BP/BP_ResourceBase.BP_ResourceBase_C|GetS_Item _asbp_resource_base))) 1)
  ;[1 1 1] Check if the item is empty
  (bind _isempty_ (Default|CheckResourceQuantity _asbp_resource_base))
  (if _isempty_
    (return true)
    (else
      (return false))))

(fn FindResources
  (params (Jobs :type Enum_Jobs%20Enum :default "NewEnumerator0"))
  (bind _resourcesfound (Variables|Default|GetresourcesFound))
  (bind _town_hall_reference (Variables|Default|GetTown%20Hall%20Reference))
  (bind _targetworkbuilding (Variables|Default|GetTargetWorkBuilding))
  (bind _output (Utilities|Array|Get(acopy) _resourcesfound))
  ;[1 1 1] Clear the previous resources
  (Utilities|Array|Clear (Variables|Default|GetresourcesFound))
  ;[1 1 1] Check if the work building is destroyed or not
  (Utilities|IsValid _targetworkbuilding
    (:Is%20Valid
      (for _array_element (Collision|GetOverlappingActors (Variables|/Game/Tools/BuildingTool/WorkBuilding/BP/BP_WorkBuildingBase.BP_WorkBuildingBase_C|GetSphereSearchArea _targetworkbuilding) "/Game/Tools/ResourceTool/BP/BP_ResourceBase.BP_ResourceBase_C" :!class /Script/Engine.PrimitiveComponent)
        (bind _asbp_resource_base (Utilities|Casting|CastToBP_ResourceBase _array_element))
        (if (and (Utilities|Enum|Equal(Enum) (.Jobs (Utilities|Struct|BreakS_Resources (Variables|/Game/Tools/ResourceTool/BP/BP_ResourceBase.BP_ResourceBase_C|GetS_Item _asbp_resource_base))) Jobs) (< (.Value (Utilities|Map|Find (Variables|/Game/Tools/BuildingTool/TownHallBuilding/BP/BP_TownHall.BP_TownHall_C|GetResourceMap _town_hall_reference) (Utilities|String|ToString(Name) (.Name (Utilities|Struct|BreakS_Resources (Variables|/Game/Tools/ResourceTool/BP/BP_ResourceBase.BP_ResourceBase_C|GetS_Item _asbp_resource_base)))))) (Variables|/Game/Tools/BuildingTool/TownHallBuilding/BP/BP_TownHall.BP_TownHall_C|GetmaxResources _town_hall_reference)))
          (Utilities|Array|AddUnique (Variables|Default|GetresourcesFound) _array_element)))
      (if (Utilities|Array|IsEmpty (Variables|Default|GetresourcesFound))
        (return false)
        (else
          (Variables|Vector|Setdestination (Transformation|GetActorLocation _output))
          (Variables|Default|SetItemToCollect _output)
          (return true))))
    (:Is%20Not%20Valid
      (CallFunction|RandomLocationWithoutWorkBuilding))))

(fn RemoveHunger
  (params (Hunger :type Integer))
  (Variables|BasicStats|SetHunger (- (Variables|BasicStats|GetHunger) Hunger)))

(fn CheckHunger
  (params (hungerAlert :type Integer) (quantityToAddAlert :type Integer))
  (LocalVariables|SetquantityToAdd quantityToAddAlert)
  (if (<= (Variables|BasicStats|GetHunger) hungerAlert)
    (bind _returnvalue (Utilities|GetDataTableRow "/Game/Tools/ResourceTool/Datatable/DT_Resources.DT_Resources" "Wheat")
      (:then
        (if (and (.ReturnValue (Utilities|Map|Find (Variables|/Game/Tools/BuildingTool/TownHallBuilding/BP/BP_TownHall.BP_TownHall_C|GetResourceMap (Variables|Default|GetTown%20Hall%20Reference)) (Utilities|String|ToString(Name) (.Name (Utilities|Struct|BreakS_Resources _returnvalue))))) (>= (.Value (Utilities|Map|Find (Variables|/Game/Tools/BuildingTool/TownHallBuilding/BP/BP_TownHall.BP_TownHall_C|GetResourceMap (Variables|Default|GetTown%20Hall%20Reference)) (Utilities|String|ToString(Name) (.Name (Utilities|Struct|BreakS_Resources _returnvalue))))) (LocalVariables|GetquantityToAdd)))
          (Utilities|Map|Add (Variables|/Game/Tools/BuildingTool/TownHallBuilding/BP/BP_TownHall.BP_TownHall_C|GetResourceMap (Variables|Default|GetTown%20Hall%20Reference)) (Utilities|String|ToString(Name) (.Name (Utilities|Struct|BreakS_Resources _returnvalue))) (- (.Value (Utilities|Map|Find (Variables|/Game/Tools/BuildingTool/TownHallBuilding/BP/BP_TownHall.BP_TownHall_C|GetResourceMap (Variables|Default|GetTown%20Hall%20Reference)) (Utilities|String|ToString(Name) (.Name (Utilities|Struct|BreakS_Resources _returnvalue))))) (LocalVariables|GetquantityToAdd)))
          (Hunger|AddHunger (LocalVariables|GetquantityToAdd)))))))

(fn AddHunger
  (params (quantityToAdd :type Integer))
  (Variables|BasicStats|SetHunger (+ (Variables|BasicStats|GetHunger) quantityToAdd)))

(fn ClearCharacterInventory
  (Utilities|Map|Clear (Variables|BasicStats|GetresourceInventory)))