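; Player controller for the character pawn that shows the menu widget and makes the navigation bounds follow the controlled pawn.
; Five seconds after BeginPlay it attaches the first NavMeshBoundsVolume to the pawn and makes its brush visible in game.
; A Delay on Tick notifies the navigation system roughly every ten seconds that the bounds changed, so navigation can update around the moving pawn.
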(event EventBeginPlay
  (bind _returnvalue (UserInterface|CreateWidget "/Game/Utilities/Widgets/WBP_Menu.WBP_Menu_C"))
  (UserInterface|Viewport|AddtoViewport _returnvalue 0)
  (Utilities|FlowControl|Delay 5.0)
  (CallFunction|SetupNavMesh))

(event EventTick
  (params (DeltaSeconds :type Float%20%28single-precision%29))
  (Utilities|FlowControl|Delay 1e+01)
  (Class|NavigationSystemV1|OnNavigationBoundsUpdated (Class|NavigationSystemV1|GetNavigationSystem) (Variables|Default|GetNavMeshB)))

(fn ConstructionScript)

(fn SetupNavMesh
  (bind _outactors (Actor|GetAllActorsOfClass "/Script/NavigationSystem.NavMeshBoundsVolume"))
  (bind _output_get (Variables|Default|SetNavMeshB (Utilities|Array|Get(acopy) _outactors)))
  (Transformation|AttachActorToActor _output_get (Pawn|GetControlledPawn) "None" "SnapToTarget" "KeepRelative" "KeepRelative" true)
  (Development|SetHiddeninGame (Variables|/Script/Engine.Brush|GetBrushComponent (Utilities|Array|Get(acopy) _outactors)) false false))