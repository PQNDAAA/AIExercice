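; Player pawn for a building game, handling camera movement, rotation, zoom, speed and Town Hall centering.
; Construction mode moves buildings to the cursor trace and rotates them with R; placing clears overlapping resources, charging the Town Hall only first time.
; X toggles a test excavate/paint actor that follows the cursor, with collision toggled by left-click.
; Both modes update through Delay loops; right-click opens resource info widgets for tagged buildings and the Town Hall.
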(event Custom|ConstructionModeRealTime
  (params (Actor%20 :type Actor%20Object%20Reference))
  ;[1 1 1] Different Functions in the Construction Mode to run it
  (Variables|ConstructionMode|SetcurrentActorInConstructionMode Actor%20)
  (bind _location (CallFunction|ForwardRaycast))
  (CallFunction|MoveActor Actor%20 (Math|Vector|MakeVector (.x _location) (.y _location) (.z _location))))

(event Custom|ConstructionModeLoop
  (params (Actor%20 :type Actor%20Object%20Reference))
  ;[1 1 1] The construction mode loop in runtime
  (Utilities|FlowControl|Delay 0.05 :!label _label)
  (if (Variables|ConstructionMode|GetConstructionMode)
    (CallFunction|ConstructionModeRealTime Actor%20)
    (goto _label)))

(event Custom|EditModeRealTime
  (bind _returnvalue (Game|GetPlayerController 0))
  (bind _hitresult (Game|Player|GetHitResultUnderCursorbyChannel _returnvalue "TraceTypeQuery1" true))
  (bind (_bblockinghit _binitialoverlap _time _distance _location _impactpoint) (Collision|BreakHitResult _hitresult))
  (bind _returnvalue_2 (Math|Vector|MakeVector (.x _location) (.y _location) (.z _impactpoint)))
  (Utilities|IsValid (Variables|EditMode|GeteditModeExcavateReference) :!label _label
    (:Is%20Valid
      (Utilities|FlowControl|Delay 0.05)
      (CallFunction|MoveActor (Variables|EditMode|GeteditModeExcavateReference) (Math|Vector|MakeVector (.x _returnvalue_2) (.y _returnvalue_2) (.z _returnvalue_2)))
      (goto _label))))

(event EventTick
  (params (DeltaSeconds :type Float%20%28single-precision%29))
  (Utilities|FlowControl|Sequence
    (:then_0
      ;[1 1 1] CameraMovement
      (Utilities|FlowControl|Gate true
        (:Exit
          (CallFunction|CameraMovement))))))

(event Input|ActionEvents|InputActionZoomIn
  (params (Key :type Key%20Structure :default "None"))
  (bind _springarm (Variables|Default|GetSpringArm))
  ;[1 1 1] Zoom Camera
  (:Pressed
    (Variables|/Script/Engine.SpringArmComponent|SetTargetArmLength _springarm (Math|Float|Clamp(Float) (- (Variables|/Script/Engine.SpringArmComponent|GetTargetArmLength _springarm) 1e+02) 0.0 5e+03))))

(event Input|ActionEvents|InputActionCenterCamera
  (params (Key :type Key%20Structure :default "None"))
  ;[1 1 1] Center the camera on the TH
  (:Pressed
    (bind (_find_ _townhallreference) (CallFunction|FindTownHall))
    (if _find_
      (Class|CharacterPawn|CenterCamera (Transformation|GetWorldLocation (Variables|/Game/Tools/BuildingTool/SimpleBuilding/BP/BP_Building.BP_Building_C|GetStaticMesh _townhallreference)) (Variables|Default|GetSpringArm)))))

(event Input|ActionEvents|InputActionZoomOut
  (params (Key :type Key%20Structure :default "None"))
  (bind _springarm (Variables|Default|GetSpringArm))
  ;[1 1 1] Zoom Camera
  (:Pressed
    (Variables|/Script/Engine.SpringArmComponent|SetTargetArmLength _springarm (Math|Float|Clamp(Float) (+ (Variables|/Script/Engine.SpringArmComponent|GetTargetArmLength _springarm) 1e+02) 0.0 5e+03))))

(event Input|ActionEvents|InputActionSpeedMovementDown
  (params (Key :type Key%20Structure :default "None"))
  (bind _floatingpawnmovement (Variables|Default|GetFloatingPawnMovement))
  ;[1 1 1] Speed Movement
  (:Pressed
    (bind _output_get (Variables|/Script/Engine.FloatingPawnMovement|SetMaxSpeed _floatingpawnmovement (Math|Float|Clamp(Float) (- (Variables|/Script/Engine.FloatingPawnMovement|GetMaxSpeed _floatingpawnmovement) 1e+02) 6e+02 2e+03)))
    (Development|PrintString (Utilities|String|ToString(Float) _output_get))))

(event Input|ActionEvents|InputActionSpeedMovementUp
  (params (Key :type Key%20Structure :default "None"))
  (bind _floatingpawnmovement (Variables|Default|GetFloatingPawnMovement))
  ;[1 1 1] Speed Movement
  (:Pressed
    (bind _output_get (Variables|/Script/Engine.FloatingPawnMovement|SetMaxSpeed _floatingpawnmovement (Math|Float|Clamp(Float) (+ (Variables|/Script/Engine.FloatingPawnMovement|GetMaxSpeed _floatingpawnmovement) 1e+02) 6e+02 2e+03)))
    (Development|PrintString (Utilities|String|ToString(Float) _output_get))))

(event Input|AxisEvents|InputAxisMoveForward/Backward
  (params (AxisValue :type Float%20%28single-precision%29))
  ;[1 1 1] Movements
  (Pawn|Input|AddMovementInput (Math|Vector|GetForwardVector (Math|Rotator|MakeRotator 0.0 0.0 (.Yaw (Math|Rotator|BreakRotator (Transformation|GetWorldRotation (Variables|Default|GetCamera)))))) AxisValue false))

(event Input|AxisEvents|InputAxisMoveRight/Left
  (params (AxisValue :type Float%20%28single-precision%29))
  (bind _camera (Variables|Default|GetCamera))
  (bind _returnvalue (Transformation|GetWorldRotation _camera))
  (bind (_roll _pitch _yaw) (Math|Rotator|BreakRotator _returnvalue))
  ;[1 1 1] Movements
  (Pawn|Input|AddMovementInput (Math|Vector|GetRightVector (Math|Rotator|MakeRotator _roll 0.0 _yaw)) AxisValue false))

(event Input|MouseEvents|RightMouseButton
  (params (Key :type Key%20Structure :default "None"))
  ;[1 1 1] Hit Result
  (:Pressed
    (CallFunction|HitResultBuilding)))

(event Input|MouseEvents|MiddleMouseButton
  (params (Key :type Key%20Structure :default "None"))
  ;[1 1 1] CameraMovement
  (:Pressed
    (Utilities|FlowControl|Gate true) ; enters at Open
  )
  (:Released
    (Utilities|FlowControl|Gate true) ; enters at Close
  ))

(event Input|MouseEvents|LeftMouseButton
  (params (Key :type Key%20Structure :default "None"))
  (bind _currentactorinconstructionmode (Variables|ConstructionMode|GetcurrentActorInConstructionMode))
  ;[1 1 1] Place building
  (:Pressed
    (if (Variables|ConstructionMode|GetConstructionMode)
      (Variables|ConstructionMode|SetConstructionMode false)
      (bind _asbp_building (Utilities|Casting|CastToBP_Building (Variables|ConstructionMode|GetcurrentActorInConstructionMode)))
      (if (Variables|/Game/Tools/BuildingTool/SimpleBuilding/BP/BP_Building.BP_Building_C|GetwasAlreadyPlaced? _asbp_building)
        (bind _asbp_building_2 (Utilities|Casting|CastToBP_Building _currentactorinconstructionmode :!label _label))
        ;;[1 1 1] Destroy actors around the target building
        (Collision|SetActorEnableCollision _currentactorinconstructionmode true)
        (Default|DestroyResourceOverlapBuilding _asbp_building_2)
        (else
          (bind _asbp_building_3 (Utilities|Casting|CastToBP_Building (Variables|ConstructionMode|GetcurrentActorInConstructionMode)))
          (Variables|/Game/Tools/BuildingTool/SimpleBuilding/BP/BP_Building.BP_Building_C|SetwasAlreadyPlaced? _asbp_building_3 true)
          (bind (_find_ _townhallreference) (CallFunction|FindTownHall))
          (if _find_
            ;;[1 1 1] Substract Ressources when the buidling is placed
            (Default|SubstractResourcesTownHall _townhallreference (Variables|/Game/Tools/BuildingTool/SimpleBuilding/BP/BP_Building.BP_Building_C|GetItemRecipe _asbp_building_3))
            (goto _label))))
      (elif (Variables|EditMode|GeteditModeIsPressed)
        (Collision|SetCollisionProfileName (Variables|/Game/EditMode/TestPaintMode.TestPaintMode_C|GetBox (Variables|EditMode|GeteditModeExcavateReference)) "OverlapAllDynamic" true :!class /Script/Engine.PrimitiveComponent)
        (Development|PrintString "Hello"))))
  (:Released
    (if (Variables|EditMode|GeteditModeIsPressed)
      (Collision|SetCollisionEnabled (Variables|/Game/EditMode/TestPaintMode.TestPaintMode_C|GetBox (Variables|EditMode|GeteditModeExcavateReference)) "NoCollision"))))

(event Input|KeyboardEvents|R
  (params (Key :type Key%20Structure :default "None"))
  ;[1 1 1] Rotate an actor in runtime with the construction mode
  (:Pressed
    (Variables|Default|SetisKeyPressed true)
    (Utilities|FlowControl|Delay 0.05 :!label _label)
    (if (and (Variables|ConstructionMode|GetConstructionMode) (Variables|Default|GetisKeyPressed))
      (CallFunction|RotateActor (Variables|ConstructionMode|GetcurrentActorInConstructionMode))
      (goto _label)))
  (:Released
    (Variables|Default|SetisKeyPressed false)))

(event Input|KeyboardEvents|SpaceBar
  (params (Key :type Key%20Structure :default "None"))
  ;[1 1 1] Debug for the Levelling System
  (:Pressed
    (Default|AddExp (Variables|Default|GetLevellingComponent) 1e+02 1)))

(event Input|KeyboardEvents|X
  (params (Key :type Key%20Structure :default "None"))
  ;[1 1 1] EditMode FlipFlop
  (:Pressed
    (if (not (Variables|ConstructionMode|GetConstructionMode))
      (Utilities|FlowControl|FlipFlop
        (:A
          (Variables|EditMode|SeteditModeIsPressed true)
          (CallFunction|SpawnEditMode)
          (Development|PrintString "EditMode is enabled")
          (CallFunction|EditModeRealTime))
        (:B
          (Variables|EditMode|SeteditModeIsPressed false)
          (Actor|DestroyActor (Variables|EditMode|GeteditModeExcavateReference))
          (Development|PrintString "EditMode is disabled"))))))

(fn ConstructionScript)

(fn CameraMovement
  (bind _springarm (Variables|Default|GetSpringArm))
  (bind _returnvalue (Transformation|GetWorldRotation _springarm))
  (bind (_roll _pitch _yaw) (Math|Rotator|BreakRotator _returnvalue))
  ;[1 1 1] Set New World Rotation
  (Transformation|SetWorldRotation (Variables|Default|GetSpringArm) (Math|Rotator|MakeRotator _roll (Math|Float|Clamp(Float) (+ _pitch (Class|Actor|GetInputAxisKeyValue)) -6e+01 -5e+01) (+ _yaw (Class|Actor|GetInputAxisKeyValue))) false false))

(fn HitResultBuilding
  (bind _returnvalue (Game|GetPlayerController 0))
  (bind _hitresult (Game|Player|GetHitResultUnderCursorbyChannel _returnvalue "TraceTypeQuery1" true))
  (bind _hitactor (Collision|BreakHitResult _hitresult))
  (if (and (!= (UserInterface|Viewport|IsinViewport (Variables|Default|GetItemsInformations_Reference)) true) (Actor|ActorHasTag _hitactor "Building"))
    ;[1 1 1] Crete the widget of informations for the building
    (bind _returnvalue_2 (UserInterface|CreateWidget "/Game/Utilities/Widgets/WBP_ObjectInformations.WBP_ObjectInformations_C" 0 _hitactor))
    (bind _output_get (Variables|Default|SetItemsInformations_Reference _returnvalue_2))
    (UserInterface|Viewport|AddtoViewport _output_get 0)
    (bind _asbp_building (Utilities|Casting|CastToBP_Building _hitactor))
    (Rendering|Components|TextRender|SetText (Variables|/Game/Utilities/Widgets/WBP_ObjectInformations.WBP_ObjectInformations_C|GetItemName (Variables|Default|GetItemsInformations_Reference)) (Utilities|Text|ToText(Name) (Variables|/Game/Tools/BuildingTool/SimpleBuilding/BP/BP_Building.BP_Building_C|GetbuildingName _asbp_building)))
    (bind _asbp_work_building_base (Utilities|Casting|CastToBP_WorkBuildingBase _asbp_building))
    (bind _keys (Utilities|Map|Keys (Variables|/Game/Tools/BuildingTool/WorkBuilding/BP/BP_WorkBuildingBase.BP_WorkBuildingBase_C|GetresourceInventory _asbp_work_building_base)))
    (for _array_element _keys
      (bind _returnvalue_3 (Utilities|GetDataTableRow "/Game/Tools/ResourceTool/Datatable/DT_Resources.DT_Resources" (Utilities|String|StringToName _array_element))
        (:then
          (bind _returnvalue_4 (UserInterface|CreateWidget "/Game/Utilities/Widgets/WBP_ObjectInformationsSlots.WBP_ObjectInformationsSlots_C"))
          (bind _output_get_2 (LocalVariables|SetNewSlotsItem _returnvalue_4))
          ;;[1 1 1] Attach the Informations to WrapBox
          (Class|WrapBox|AddChildtoWrapBox (Variables|/Game/Utilities/Widgets/WBP_ObjectInformations.WBP_ObjectInformations_C|GetSlotsPanel (Variables|Default|GetItemsInformations_Reference)) _output_get_2)
          (Rendering|Components|TextRender|SetText (Variables|/Game/Utilities/Widgets/WBP_ObjectInformationsSlots.WBP_ObjectInformationsSlots_C|Getquantity (LocalVariables|GetNewSlotsItem)) (Utilities|Text|ToText(Integer) (.Value (Utilities|Map|Find (Variables|/Game/Tools/BuildingTool/WorkBuilding/BP/BP_WorkBuildingBase.BP_WorkBuildingBase_C|GetresourceInventory _asbp_work_building_base) _array_element))))
          ;;[1 1 1] Set Resource Logo
          (Default|SetImage (LocalVariables|GetNewSlotsItem) (.Image (Utilities|Struct|BreakS_Resources _returnvalue_3))))))
    (bind _returnvalue_5 (UserInterface|CreateWidget "/Game/Utilities/Widgets/WBP_ObjectInformationsSlots.WBP_ObjectInformationsSlots_C"))
    (bind _output_get_3 (LocalVariables|SetNewSlotsItem _returnvalue_5))
    (Class|WrapBox|AddChildtoWrapBox (Variables|/Game/Utilities/Widgets/WBP_ObjectInformations.WBP_ObjectInformations_C|GetSlotsPanel (Variables|Default|GetItemsInformations_Reference)) _output_get_3)
    (Rendering|Components|TextRender|SetText (Variables|/Game/Utilities/Widgets/WBP_ObjectInformationsSlots.WBP_ObjectInformationsSlots_C|Getquantity (LocalVariables|GetNewSlotsItem)) (Utilities|Text|FormatText "Character: {Min}/{Max}" (Variables|/Game/Tools/BuildingTool/WorkBuilding/BP/BP_WorkBuildingBase.BP_WorkBuildingBase_C|GetcurrentVillagers _asbp_work_building_base) (Variables|/Game/Tools/BuildingTool/WorkBuilding/BP/BP_WorkBuildingBase.BP_WorkBuildingBase_C|GetvillagersMax _asbp_work_building_base)))
    (Variables|/Script/UMG.TextLayoutWidget|SetJustification (Variables|/Game/Utilities/Widgets/WBP_ObjectInformationsSlots.WBP_ObjectInformationsSlots_C|Getquantity (LocalVariables|GetNewSlotsItem)) "Left")
    (elif (and (!= (UserInterface|Viewport|IsinViewport (Variables|Default|GetItemsInformations_Reference)) true) (Actor|ActorHasTag _hitactor "TownHall"))
      ;[1 1 1] Create the widget of Informations for the TownHall
      (bind _returnvalue_6 (UserInterface|CreateWidget "/Game/Utilities/Widgets/WBP_ObjectInformations.WBP_ObjectInformations_C" 0 _hitactor))
      (bind _output_get_4 (Variables|Default|SetItemsInformations_Reference _returnvalue_6))
      (UserInterface|Viewport|AddtoViewport _output_get_4 0)
      (bind _asbp_town_hall (Utilities|Casting|CastToBP_TownHall _hitactor))
      ;;[1 1 1] Get Resource String to identify them
      (bind _keys_2 (Utilities|Map|Keys (Variables|/Game/Tools/BuildingTool/TownHallBuilding/BP/BP_TownHall.BP_TownHall_C|GetResourceMap _asbp_town_hall)))
      (for _array_element_2 _keys_2
        (bind _returnvalue_7 (Utilities|GetDataTableRow "/Game/Tools/ResourceTool/Datatable/DT_Resources.DT_Resources" (Utilities|String|StringToName _array_element_2))
          (:then
            (bind _returnvalue_8 (UserInterface|CreateWidget "/Game/Utilities/Widgets/WBP_ObjectInformationsSlots.WBP_ObjectInformationsSlots_C"))
            (bind _output_get_5 (LocalVariables|SetNewSlotsItem _returnvalue_8))
            ;;[1 1 1] Attach the informations to WrapBox
            (Class|WrapBox|AddChildtoWrapBox (Variables|/Game/Utilities/Widgets/WBP_ObjectInformations.WBP_ObjectInformations_C|GetSlotsPanel (Variables|Default|GetItemsInformations_Reference)) _output_get_5)
            (Rendering|Components|TextRender|SetText (Variables|/Game/Utilities/Widgets/WBP_ObjectInformations.WBP_ObjectInformations_C|GetItemName (Variables|Default|GetItemsInformations_Reference)) (Utilities|Text|ToText(Name) (Variables|/Game/Tools/BuildingTool/SimpleBuilding/BP/BP_Building.BP_Building_C|GetbuildingName _asbp_town_hall)))
            (Rendering|Components|TextRender|SetText (Variables|/Game/Utilities/Widgets/WBP_ObjectInformationsSlots.WBP_ObjectInformationsSlots_C|Getquantity (LocalVariables|GetNewSlotsItem)) (Utilities|Text|ToText(Integer) (.Value (Utilities|Map|Find (Variables|/Game/Tools/BuildingTool/TownHallBuilding/BP/BP_TownHall.BP_TownHall_C|GetResourceMap _asbp_town_hall) _array_element_2))))
            ;;[1 1 1] Set Resource Logo
            (Default|SetImage (LocalVariables|GetNewSlotsItem) (.Image (Utilities|Struct|BreakS_Resources _returnvalue_7)))
            (Widget|SetVisibility (Variables|/Game/Utilities/Widgets/WBP_ObjectInformations.WBP_ObjectInformations_C|GetDestroyBtn (Variables|Default|GetItemsInformations_Reference)) "Hidden")))))))

(fn ForwardRaycast
  (params (Target :type Scene%20Component%20Object%20Reference))
  (bind _returnvalue (Game|GetPlayerController 0))
  (bind _hitresult (Game|Player|GetHitResultUnderCursorbyChannel _returnvalue "TraceTypeQuery1" true))
  (bind (_bblockinghit _binitialoverlap _time _distance _location _impactpoint) (Collision|BreakHitResult _hitresult))
  (return (Math|Vector|MakeVector (.x _location) (.y _location) (.z _impactpoint))))

(fn MoveActor
  (params (Actor :type Actor%20Object%20Reference) (Location :type Vector))
  (Transformation|SetActorLocation Actor Location false false))

(fn RotateActor
  (params (Target :type Actor%20Object%20Reference))
  (bind _returnvalue (Transformation|GetActorRotation Target))
  ;[1 1 1] Rotate an actor in runtime until 360° by adding 10°
  (if (>= (.yaw _returnvalue) 3.6e+02)
    (Transformation|SetActorRotation Target)
    (else
      (Transformation|SetActorRotation Target (Math|Rotator|MakeRotator (.roll _returnvalue) (.pitch _returnvalue) (+ (.yaw _returnvalue) 1e+01))))))

(fn SpawnEditMode
  (bind _returnvalue (Game|GetPlayerController 0))
  (bind _hitresult (Game|Player|GetHitResultUnderCursorbyChannel _returnvalue "TraceTypeQuery1" true))
  (bind _location (Collision|BreakHitResult _hitresult))
  (Development|PrintString (Utilities|String|ToString(Vector) _location))
  (bind _returnvalue_2 (Game|SpawnActorfromClass "/Game/EditMode/TestPaintMode.TestPaintMode_C" (Math|Transform|MakeTransform _location "0, 0, 0" "1.000000,1.000000,1.000000") "Undefined" 0 0))
  (bind _output_get (Variables|EditMode|SeteditModeExcavateReference _returnvalue_2))
  (Collision|SetCollisionEnabled (Variables|/Game/EditMode/TestPaintMode.TestPaintMode_C|GetBox _output_get) "NoCollision"))