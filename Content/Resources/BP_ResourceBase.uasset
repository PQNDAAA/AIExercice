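; BP_ResourceBase is a base Blueprint for world resources, configured from an item data table row.
; The Construction Script looks up the Item row handle, caches it as SItem and applies its static mesh.
; It also adds the row's item quantity to the existing ResourceInventory value rather than overwriting it.
; The event graph holds only disabled stub events, so no runtime behavior is defined here.
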(event EventBeginPlay)

(event Collision|EventActorBeginOverlap
  (params (OtherActor :type Actor%20Object%20Reference)))

(event EventTick
  (params (DeltaSeconds :type Float%20%28single-precision%29)))

(fn ConstructionScript
  (bind _item (Variables|Default|GetItem))
  (bind (_datatable _rowname) (Utilities|Struct|BreakDataTableRowHandle _item))
  (bind _returnvalue (Utilities|GetDataTableRow _datatable _rowname)
    (:then
      (Variables|Default|SetS_Item _returnvalue)
      (Components|StaticMesh|SetStaticMesh (Variables|Default|GetStaticMesh) (.StaticMesh (Utilities|Struct|BreakS_Resources (Variables|Default|GetS_Item))))
      (Variables|Default|SetresourceInventory (+ (Variables|Default|GetresourceInventory) (.ItemQuantity (Utilities|Struct|BreakS_Resources (Variables|Default|GetS_Item))))))))