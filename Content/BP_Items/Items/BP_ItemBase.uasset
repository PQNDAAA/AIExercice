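; BP_ItemBase is a base item actor with a static mesh and a villager count limited by a maximum.
; Its construction script applies StaticMeshReference to the mesh and prints VillagersMax; unconnected data table and render target nodes never run.
; AddPeople and ReducePeople adjust CurrentVillagers without clamping, while CheckCapacity separately reports whether it is below VillagersMax.
; The event graph has no active logic.
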(event EventBeginPlay)

(event Collision|EventActorBeginOverlap
  (params (OtherActor :type Actor%20Object%20Reference)))

(event EventTick
  (params (DeltaSeconds :type Float%20%28single-precision%29)))

(fn ConstructionScript
  (Components|StaticMesh|SetStaticMesh (Variables|Default|GetStaticMesh) (Variables|Default|GetStatic_Mesh_Reference))
  (Development|PrintString (Utilities|String|ToString(Integer) (Variables|Informations|GetvillagersMax))))

(fn AddPeople
  (params (value :type Integer))
  (Variables|Informations|SetcurrentVillagers (+ value (Variables|Informations|GetcurrentVillagers))))

(fn CheckCapacity
  (if (< (Variables|Informations|GetcurrentVillagers) (Variables|Informations|GetvillagersMax))
    (return true)
    (else
      (return false))))

(fn ReducePeople
  (params (value :type Integer))
  (Variables|Informations|SetcurrentVillagers (- (Variables|Informations|GetcurrentVillagers) value)))