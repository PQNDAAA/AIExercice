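; Villager AI character that joins a storage building matching its job, gathers resources there and manages hunger.
; Self-recalling Blueprint events chain AIMoveTo to harvest resources below town hall caps, award player XP, deposit and rest, wandering when idle.
; Tick re-searches when targets deplete and refreshes the drop-off point during construction mode.
; A parallel hunger loop eats town hall Wheat and destroys the villager at zero.
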(event Custom|GoToBase
  (Variables|Boolean|SetinBase true)
  (Variables|Boolean|SetisGoingAtWork? false)
  (AI|AIMoveTo self (Variables|Vector|GetstorageBuildingDestination) 0 1e+02 false
    (:OnSuccess
      (bind _playerinventoryclear (CallFunction|ResourcetoAdd (Variables|BasicStats|GetresourceInventory) (Variables|Default|GetTargetStorageBuilding)))
      (Variables|BasicStats|SetresourceInventory _playerinventoryclear)
      (Utilities|FlowControl|Delay (Variables|BasicStats|GetDurationForBreak))
      (Variables|Boolean|SetinBase false)
      (CallFunction|SearchWork))))

(event Custom|RandomLocationWithoutBase
  (AI|AIMoveTo self (.RandomLocation (AI|Navigation|GetRandomReachablePointinRadius (Transformation|GetActorLocation) 4e+02 0 0)) 0 5e+01 false
    (:OnSuccess
      _)
    (:OnFail
      _))
  (Utilities|FlowControl|Delay 1.0)
  (bind _isfound_ (CallFunction|SearchBuilding))
  (if _isfound_
    (CallFunction|SearchWork)
    (else
      (CallFunction|RandomLocationWithoutBase))))

(event Custom|GoToWork
  (Variables|Boolean|SetisGoingAtWork? true)
  (AI|AIMoveTo self (Variables|Vector|Getdestination) 0 3e+01 false
    (:OnSuccess
      (bind _isempty_ (CallFunction|AddResourceInventory (Variables|Default|GetItemToCollect)))
      (if _isempty_
        (Default|DestroyInstancedStaticMeshTreeComponent (CallFunction|GetMap) (Variables|Default|GetItemToCollect)))
      (CallFunction|GotoBase))))

(event Custom|RandomLocation
  (if (and (== (Variables|Boolean|GetisGoingAtWork?) false) (== (Variables|Boolean|GetinBase) false))
    (AI|AIMoveTo self (.RandomLocation (AI|Navigation|GetRandomReachablePointinRadius (Transformation|GetActorLocation (Variables|Default|GetTargetStorageBuilding)) (/ (Variables|BasicStats|GetsearchArea) 2.0) 0 0)) 0 5e+01 false
      (:OnSuccess
        _)
      (:OnFail
        _))
    (Utilities|FlowControl|Delay 1.0)
    (CallFunction|SearchWork)
    (else
      (Utilities|FlowControl|Delay 0.2)
      (CallFunction|RandomLocation))))

(event Custom|HungerUpdate
  (if (<= (Variables|BasicStats|GetHunger) 0)
    (Default|ReducePeople (Variables|Default|GetTargetStorageBuilding) 1)
    (Actor|DestroyActor)
    (else
      (Utilities|FlowControl|Delay 2.0)
      (CallFunction|RemoveHunger 2)
      (CallFunction|CheckHunger 70 10)
      (CallFunction|HungerUpdate))))

(event Custom|SearchWork
  (Variables|Boolean|SetisGoingAtWork? false)
  (bind _found_ (CallFunction|FindResources (Variables|BasicStats|GetJobs)))
  (if _found_
    (CallFunction|GotoWork)
    (else
      (CallFunction|RandomLocation))))

(event EventBeginPlay
  (Utilities|FlowControl|Delay 1.0)
  (CallFunction|SetWidgetName (Variables|Default|GetWidget))
  (CallFunction|HungerUpdate)
  (bind _isfound_ (CallFunction|SearchBuilding))
  (if _isfound_
    (CallFunction|SearchWork)
    (else
      (CallFunction|RandomLocationWithoutBase))))

(event EventTick
  (params (DeltaSeconds :type Float%20%28single-precision%29))
  (bind _targetstoragebuilding (Variables|Default|GetTargetStorageBuilding))
  (Utilities|FlowControl|Sequence
    (:then_0
      (bind _isempty_ (CallFunction|CheckQuantityItem (Variables|Default|GetItemToCollect)))
      (if (and _isempty_ (Variables|Boolean|GetisGoingAtWork?))
        (CallFunction|SearchWork)))
    (:then_1
      (bind _asbp_character_pawn (Utilities|Casting|CastToBP_CharacterPawn (Game|Player|GetPlayerPawn 0)))
      (if (Variables|/Game/ThirdPerson/Blueprints/BP_CharacterPawn.BP_CharacterPawn_C|GetConstructionMode _asbp_character_pawn)
        (Utilities|IsValid _targetstoragebuilding
          (:Is%20Valid
            (Variables|Vector|SetstorageBuildingDestination (Transformation|GetWorldLocation (Variables|/Game/Building/StorageBuilding/BP_StorageBuildingBase.BP_StorageBuildingBase_C|GetPoint _targetstoragebuilding)))))))))

(fn ConstructionScript
  (Variables|/Script/Engine.CharacterMovementComponent|SetMaxWalkSpeed (Variables|Character|GetCharacterMovement) (Variables|BasicStats|GetdefaultValueSpeed)))

(fn CheckLocation
  (params (PlayerLocation :type Vector) (Destination%20Location :type Vector))
  (bind _returnvalue (- PlayerLocation Destination%20Location))
  (return (Math|Boolean|ANDBoolean (<= (.x _returnvalue) 1e+02) (>= (.x _returnvalue) -1e+02) (<= (.y _returnvalue) 1e+02) (>= (.y _returnvalue) -1e+02))))

(fn SearchBuilding
  (LocalVariables|SethasFound? false)
  (bind _outactors (Actor|GetAllActorsOfClass "/Game/Building/StorageBuilding/BP_StorageBuildingBase.BP_StorageBuildingBase_C"))
  (bind _array_element (Utilities|Array|ForEachLoopwithBreak _outactors)
    (:LoopBody
      (if (Math|Boolean|ANDBoolean (== (Utilities|Array|Get(acopy) (Variables|/Script/Engine.Actor|GetTags _array_element)) "Building") (CallFunction|CheckStorageBuildingJobs _array_element (Variables|BasicStats|GetJobs)) (CallFunction|CheckStorageBuildingCapacity _array_element))
        (LocalVariables|SethasFound? true)
        (bind _output_get (Variables|Default|SetTargetStorageBuilding _array_element))
        (Variables|Vector|SetstorageBuildingDestination (Transformation|GetWorldLocation (Variables|/Game/Building/StorageBuilding/BP_StorageBuildingBase.BP_StorageBuildingBase_C|GetPoint (Variables|Default|GetTargetStorageBuilding))))
        (Variables|BasicStats|SetsearchArea (Variables|/Game/Building/StorageBuilding/BP_StorageBuildingBase.BP_StorageBuildingBase_C|GetsearchArea _output_get))
        (Default|AddPeople (Variables|Default|GetTargetStorageBuilding) 1)
        (return (LocalVariables|GethasFound?))))
    (:Completed
      (if (== (LocalVariables|GethasFound?) false)
        (return (LocalVariables|GethasFound?))))))

(fn SetWidgetName
  (params (Widget :type Widget%20Component%20Object%20Reference))
  (bind _aswbp_character_bar_name (Utilities|Casting|CastToWBP_CharacterBarName (UserInterface|GetUserWidgetObject Widget)))
  (Rendering|Components|TextRender|SetText (Variables|/Game/Widget/WBP_CharacterBarName.WBP_CharacterBarName_C|GetnameText _aswbp_character_bar_name) (Utilities|Text|ToText(String) (Utilities|String|ToString(Name) (Variables|BasicStats|GetName)))))

(fn AddResourceInventory
  (params (Item :type Actor%20Object%20Reference))
  (bind _asbp_resource_base (Utilities|Casting|CastToBP_ResourceBase Item))
  (Utilities|Map|Add (Variables|BasicStats|GetresourceInventory) (Utilities|String|ToString(Name) (.Name (Utilities|Struct|BreakS_Resources (Variables|/Game/Resources/BP_ResourceBase.BP_ResourceBase_C|GetS_Item _asbp_resource_base)))) 1)
  (Variables|/Game/Resources/BP_ResourceBase.BP_ResourceBase_C|SetresourceInventory _asbp_resource_base (- (Variables|/Game/Resources/BP_ResourceBase.BP_ResourceBase_C|GetresourceInventory _asbp_resource_base) 1))
  (bind _asbp_character_pawn (Utilities|Casting|CastToBP_CharacterPawn (Game|Player|GetPlayerPawn 0)))
  (Default|AddExp (Variables|/Game/ThirdPerson/Blueprints/BP_CharacterPawn.BP_CharacterPawn_C|GetLevellingComponent _asbp_character_pawn) (.RewardExp (Utilities|Struct|BreakS_Resources (Variables|/Game/Resources/BP_ResourceBase.BP_ResourceBase_C|GetS_Item _asbp_resource_base))) 1)
  (bind _isempty_ (CallFunction|CheckQuantityItem Item))
  (if _isempty_
    (return true)
    (else
      (return false))))

(fn FindResources
  (params (Jobs :type Enum_Jobs%20Enum :default "NewEnumerator0"))
  (bind _resourcesfound (Variables|Default|GetresourcesFound))
  (bind _output (Utilities|Array|Get(acopy) _resourcesfound))
  (bind (_find_ _townhallreference) (CallFunction|FindTownHall))
  (if _find_
    (Variables|Default|SetTown%20Hall%20Reference _townhallreference)
    (Utilities|Array|Clear (Variables|Default|GetresourcesFound))
    (for _array_element (Collision|GetOverlappingActors (Variables|/Game/Building/StorageBuilding/BP_StorageBuildingBase.BP_StorageBuildingBase_C|GetSphereSearchArea (Variables|Default|GetTargetStorageBuilding)) "/Game/Resources/BP_ResourceBase.BP_ResourceBase_C" :!class /Script/Engine.PrimitiveComponent)
      (bind _asbp_resource_base (Utilities|Casting|CastToBP_ResourceBase _array_element))
      (if (and (Utilities|Enum|Equal(Enum) (.Jobs (Utilities|Struct|BreakS_Resources (Variables|/Game/Resources/BP_ResourceBase.BP_ResourceBase_C|GetS_Item _asbp_resource_base))) Jobs) (< (.Value (Utilities|Map|Find (Variables|/Game/BP_TownHall/BP_TownHall.BP_TownHall_C|GetResourceMap (Variables|Default|GetTown%20Hall%20Reference)) (Utilities|String|ToString(Name) (.Name (Utilities|Struct|BreakS_Resources (Variables|/Game/Resources/BP_ResourceBase.BP_ResourceBase_C|GetS_Item _asbp_resource_base)))))) (Variables|/Game/BP_TownHall/BP_TownHall.BP_TownHall_C|GetmaxResources (Variables|Default|GetTown%20Hall%20Reference))))
        (Utilities|Array|AddUnique (Variables|Default|GetresourcesFound) _array_element)))
    (if (Utilities|Array|IsEmpty (Variables|Default|GetresourcesFound))
      (return false)
      (else
        (Variables|Vector|Setdestination (Transformation|GetActorLocation _output))
        (Variables|Default|SetItemToCollect _output)
        (return true)))))

(fn RemoveHunger
  (params (Hunger :type Integer))
  (Variables|BasicStats|SetHunger (- (Variables|BasicStats|GetHunger) Hunger)))

(fn CheckHunger
  (params (hungerAlert :type Integer) (quantityToAddAlert :type Integer))
  (LocalVariables|SetquantityToAdd quantityToAddAlert)
  (if (<= (Variables|BasicStats|GetHunger) hungerAlert)
    (bind _returnvalue (Utilities|GetDataTableRow "/Game/Resources/DT_Resources.DT_Resources" "Wheat")
      (:then
        (if (and (.ReturnValue (Utilities|Map|Find (Variables|/Game/BP_TownHall/BP_TownHall.BP_TownHall_C|GetResourceMap (Variables|Default|GetTown%20Hall%20Reference)) (Utilities|String|ToString(Name) (.Name (Utilities|Struct|BreakS_Resources _returnvalue))))) (>= (.Value (Utilities|Map|Find (Variables|/Game/BP_TownHall/BP_TownHall.BP_TownHall_C|GetResourceMap (Variables|Default|GetTown%20Hall%20Reference)) (Utilities|String|ToString(Name) (.Name (Utilities|Struct|BreakS_Resources _returnvalue))))) (LocalVariables|GetquantityToAdd)))
          (Utilities|Map|Add (Variables|/Game/BP_TownHall/BP_TownHall.BP_TownHall_C|GetResourceMap (Variables|Default|GetTown%20Hall%20Reference)) (Utilities|String|ToString(Name) (.Name (Utilities|Struct|BreakS_Resources _returnvalue))) (- (.Value (Utilities|Map|Find (Variables|/Game/BP_TownHall/BP_TownHall.BP_TownHall_C|GetResourceMap (Variables|Default|GetTown%20Hall%20Reference)) (Utilities|String|ToString(Name) (.Name (Utilities|Struct|BreakS_Resources _returnvalue))))) (LocalVariables|GetquantityToAdd)))
          (CallFunction|AddHunger (LocalVariables|GetquantityToAdd)))))))

(fn AddHunger
  (params (quantityToAdd :type Integer))
  (Variables|BasicStats|SetHunger (+ (Variables|BasicStats|GetHunger) quantityToAdd)))