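; BP_WorkBuildingBase is a base Blueprint for work buildings that tracks how many villagers are assigned to it.
; The construction script applies a configurable static mesh and sizes a sphere search area from the SearchArea variable.
; AddPeople and ReducePeople adjust CurrentVillagers without any limit checks.
; BeginPlay enables click events on the first player controller.
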(event EventBeginPlay
  (Variables|/Script/Engine.PlayerController|SetbEnableClickEvents (Game|GetPlayerController 0) true))

(fn ConstructionScript
  (|CallParentFunction)
  (Components|StaticMesh|SetStaticMesh (Variables|Default|GetStaticMesh) (Variables|Default|GetStatic_Mesh_Reference))
  (Components|Sphere|SetSphereRadius (Variables|Default|GetSphereSearchArea) (Variables|Informations|GetsearchArea) true))

(fn AddPeople
  (params (value :type Integer))
  (Variables|Informations|SetcurrentVillagers (+ value (Variables|Informations|GetcurrentVillagers))))

(fn ReducePeople
  (params (value :type Integer))
  (Variables|Informations|SetcurrentVillagers (- (Variables|Informations|GetcurrentVillagers) value)))