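; BP_Building is a building actor with a static mesh and a box sized by its placement area.
; The construction script moves the box to the mesh's relative location and sets all three extents from PlacementArea.
; A helper function moves the box to the relative location of a supplied target component.
; The event graph holds no runtime logic.
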(event EventBeginPlay)

(event Collision|EventActorBeginOverlap
  (params (OtherActor :type Actor%20Object%20Reference)))

(event EventTick
  (params (DeltaSeconds :type Float%20%28single-precision%29)))

(fn ConstructionScript
  (bind _placementarea (Variables|Default|GetplacementArea))
  (Transformation|SetRelativeLocation (Variables|Default|GetBox) (Variables|/Script/Engine.SceneComponent|GetRelativeLocation (Variables|Default|GetStaticMesh)) false false)
  (Components|Box|SetBoxExtent (Variables|Default|GetBox) (Math|Vector|MakeVector _placementarea _placementarea _placementarea) true))

(fn SetBoxLocation
  (params (Target :type Scene%20Component%20Object%20Reference))
  (Transformation|SetRelativeLocation (Variables|Default|GetBox) (Variables|/Script/Engine.SceneComponent|GetRelativeLocation Target) false false))