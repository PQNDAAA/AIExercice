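; BP_StorageBuildingBase is a base Blueprint for storage buildings that tracks a villager count.
; Its construction script runs the parent's, assigns the configured mesh, sizes a sphere search area and offsets a Point component just beyond the box's X extent.
; AddPeople and ReducePeople adjust the villager count without bounds checks.
; BeginPlay enables click events on the first player controller.
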(event EventBeginPlay
  (Variables|/Script/Engine.PlayerController|SetbEnableClickEvents (Game|GetPlayerController 0) true))

(fn ConstructionScript
  (bind _point (Variables|Default|GetPoint))
  (bind _relativelocation (Variables|/Script/Engine.SceneComponent|GetRelativeLocation _point))
  (|CallParentFunction)
  (Components|StaticMesh|SetStaticMesh (Variables|Default|GetStaticMesh) (Variables|Default|GetStatic_Mesh_Reference))
  (Components|Sphere|SetSphereRadius (Variables|Default|GetSphereSearchArea) (Variables|Informations|GetsearchArea) true)
  (Transformation|SetRelativeLocation _point (Math|Vector|MakeVector (+ (.x (Variables|/Script/Engine.BoxComponent|GetBoxExtent (Variables|Default|GetBox))) 4e+01) (.y _relativelocation) (.z _relativelocation)) false false))

(fn AddPeople
  (params (value :type Integer))
  (Variables|Informations|SetcurrentVillagers (+ value (Variables|Informations|GetcurrentVillagers))))

(fn ReducePeople
  (params (value :type Integer))
  (Variables|Informations|SetcurrentVillagers (- (Variables|Informations|GetcurrentVillagers) value)))