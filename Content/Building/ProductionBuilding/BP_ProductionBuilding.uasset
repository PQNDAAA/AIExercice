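; Production building that periodically generates one unit of its configured resource for the town hall.
; A looping delay from BeginPlay calls AddResourceInventory, which looks up the resource in DT_Resources and adds it to the town hall, clamped to its maximum capacity.
; The added amount is also recorded in the building's own inventory map and grants the player pawn scaled experience through its LevellingComponent.
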(event EventBeginPlay
  (|CallParentFunction)
  (Utilities|FlowControl|Delay (Variables|Default|GetrewardDelay) :!label _label)
  (CallFunction|AddResourceInventory 1 (Variables|Default|GetresourceToProduce))
  (goto _label))

(event Collision|EventActorBeginOverlap
  (params (OtherActor :type Actor%20Object%20Reference))
  (|CallParentFunction OtherActor) ; This node is disabled and will not be called.\nDrag off pins to build functionality.
)

(event EventTick
  (params (DeltaSeconds :type Float%20%28single-precision%29))
  (|CallParentFunction DeltaSeconds) ; This node is disabled and will not be called.\nDrag off pins to build functionality.
)

(fn ConstructionScript
  (|CallParentFunction))

(fn AddResourceInventory
  (params (Quantity :type Integer) (RowName :type Name))
  (LocalVariables|SetremainingQuantity Quantity)
  (bind _townhallreference (CallFunction|FindTownHall))
  (LocalVariables|SetTownHallReference _townhallreference)
  (bind _returnvalue (Utilities|GetDataTableRow "/Game/Resources/DT_Resources.DT_Resources" RowName)
    (:then
      (if (<= (+ (.Value (Utilities|Map|Find (Variables|/Game/BP_TownHall/BP_TownHall.BP_TownHall_C|GetResourceMap (LocalVariables|GetTownHallReference)) (Utilities|String|ToString(Name) (.Name (Utilities|Struct|BreakS_Resources _returnvalue))))) (LocalVariables|GetremainingQuantity)) (Variables|/Game/BP_TownHall/BP_TownHall.BP_TownHall_C|GetmaxResources (LocalVariables|GetTownHallReference)))
        (bind _isadded_ (CallFunction|UpdateQuantityTownHall (Utilities|String|ToString(Name) (.Name (Utilities|Struct|BreakS_Resources _returnvalue))) (LocalVariables|GetremainingQuantity)))
        (if _isadded_
          (Utilities|Map|Add (Variables|Default|GetresourceInventory) (Utilities|String|ToString(Name) (.Name (Utilities|Struct|BreakS_Resources _returnvalue))) (+ (.Value (Utilities|Map|Find (Variables|Default|GetresourceInventory) (Utilities|String|ToString(Name) (.Name (Utilities|Struct|BreakS_Resources _returnvalue))))) (LocalVariables|GetremainingQuantity)) :!label _label)
          (bind _asbp_character_pawn (Utilities|Casting|CastToBP_CharacterPawn (Game|Player|GetPlayerPawn 0)))
          (Default|AddExp (Variables|/Game/ThirdPerson/Blueprints/BP_CharacterPawn.BP_CharacterPawn_C|GetLevellingComponent _asbp_character_pawn) (.RewardExp (Utilities|Struct|BreakS_Resources _returnvalue)) (LocalVariables|GetremainingQuantity)))
        (else
          (bind _output_get (LocalVariables|SetremainingQuantity (- (LocalVariables|GetremainingQuantity) (- (+ (.Value (Utilities|Map|Find (Variables|/Game/BP_TownHall/BP_TownHall.BP_TownHall_C|GetResourceMap (LocalVariables|GetTownHallReference)) (Utilities|String|ToString(Name) (.Name (Utilities|Struct|BreakS_Resources _returnvalue))))) (LocalVariables|GetremainingQuantity)) (Variables|/Game/BP_TownHall/BP_TownHall.BP_TownHall_C|GetmaxResources (LocalVariables|GetTownHallReference))))))
          (CallFunction|UpdateQuantityTownHall (Utilities|String|ToString(Name) (.Name (Utilities|Struct|BreakS_Resources _returnvalue))) _output_get)
          (goto _label))))))