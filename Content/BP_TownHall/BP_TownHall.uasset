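; Town hall Blueprint that fills its resource storage from a virtual inventory when play begins.
; AddResourcesTownHall looks up each VirtualInventory key in DT_Resources and uses the row's Name as the resource type.
; It writes that type's amount into ResourceMap, capped at MaxResources, leaving VirtualInventory unchanged.
; Keys without a table row only print an error.
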(event EventBeginPlay
  (CallFunction|AddResourcesTownHall))

(event EventTick
  (params (DeltaSeconds :type Float%20%28single-precision%29)))

(fn ConstructionScript
  (|CallParentFunction))

(fn AddResourcesTownHall
  (bind _maxresources (Variables|Default|GetmaxResources))
  (bind _resourcemap (Variables|Default|GetResourceMap))
  (bind _keys (Utilities|Map|Keys (Variables|Default|GetvirtualInventory)))
  (for _array_element _keys
    (bind _returnvalue (Utilities|GetDataTableRow "/Game/Resources/DT_Resources.DT_Resources" (Utilities|String|StringToName _array_element))
      (:then
        (LocalVariables|SetResourceType (Utilities|String|ToString(Name) (.Name (Utilities|Struct|BreakS_Resources _returnvalue))))
        (if (< (.Value (Utilities|Map|Find (Variables|Default|GetvirtualInventory) (LocalVariables|GetResourceType))) _maxresources)
          (Utilities|Map|Add _resourcemap (LocalVariables|GetResourceType) (.Value (Utilities|Map|Find (Variables|Default|GetvirtualInventory) (LocalVariables|GetResourceType))))
          (else
            (Utilities|Map|Add _resourcemap (LocalVariables|GetResourceType) (- (.Value (Utilities|Map|Find (Variables|Default|GetvirtualInventory) (LocalVariables|GetResourceType))) (- (.Value (Utilities|Map|Find (Variables|Default|GetvirtualInventory) (LocalVariables|GetResourceType))) _maxresources))))))
      (:RowNotFound
        (Development|PrintString "Resource not found")))))