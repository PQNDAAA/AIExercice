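; Procedural terrain actor that builds a block-grid landscape with trees, rocks and optional water in its construction script.
; GenerateMap samples simplex fractal noise per cell for elevation, adding instanced ground meshes with elevation and sand height as custom data for the tinted material.
; Each cell randomly scatters trees within height limits and rocks by density, plus water below a set level.
; Helpers randomize map parameters and pick or remove tree instances.
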(event EventBeginPlay)

(event Collision|EventActorBeginOverlap
  (params (OtherActor :type Actor%20Object%20Reference)))

(event EventTick
  (params (DeltaSeconds :type Float%20%28single-precision%29)))

(fn ConstructionScript
  (GenerateMap|GenerateMap (Variables|MapConfiguration|GetSize) (Variables|MapConfiguration|GetSeed) (Variables|MapConfiguration|GetFrequency)))

(fn GenerateMap
  (params (Size :type Integer) (Seed :type Integer) (Frequency :type Float%20%28double-precision%29))
  (bind _ground (Variables|Default|GetGround))
  (bind _returnvalue (Game|ConstructObjectfromClass "/Script/FastNoiseGenerator.FastNoiseWrapper"))
  (bind _output_get (Variables|GenerateMap|SetFastNoiseWrapper _returnvalue))
  (Class|FastNoiseWrapper|SetupFastNoise _output_get "SimplexFractal" Seed Frequency "Quintic" "FBM" 2 2.0 0.5 0.45 "Natural" "CellValue")
  (for _index (range 0 Size)
    (Variables|GenerateMap|Setx (Math|Conversions|ToFloat(Integer) (- _index 1)))
    (for _index_2 (range 0 Size)
      (Variables|GenerateMap|Sety (Math|Conversions|ToFloat(Integer) (- _index_2 1)))
      (Transformation|SetWorldScale3D (Variables|Default|GetGround) (Math|Vector|MakeVector 1.0 1.0 (Variables|MapConfiguration|GetHeightMap)))
      (Variables|Default|SetElevation (* (Class|FastNoiseWrapper|GetNoise2D (Variables|GenerateMap|GetFastNoiseWrapper) (Variables|GenerateMap|Getx) (Variables|GenerateMap|Gety)) (Variables|GenerateMap|GetHeight)))
      (Variables|GenerateMap|SetTree%20Height%20Limit%20Water -1e+02)
      (bind _returnvalue_2 (Rendering|Material|CreateDynamicMaterialInstance _ground 0 "/Game/Materials/Ground_Inst.Ground_Inst" "None" :!class /Script/Engine.PrimitiveComponent))
      (Rendering|Material|SetVectorParameterValue _returnvalue_2 "Sand" (Variables|ColorConfiguration|GetSandColor) :!class /Script/Engine.MaterialInstanceDynamic)
      (Rendering|Material|SetVectorParameterValue _returnvalue_2 "Landscape" (Variables|ColorConfiguration|GetLandscape1) :!class /Script/Engine.MaterialInstanceDynamic)
      (Rendering|Material|SetVectorParameterValue _returnvalue_2 "Landscape2" (Variables|ColorConfiguration|GetLandscape2) :!class /Script/Engine.MaterialInstanceDynamic)
      (Variables|GenerateMap|SetGridVector (Math|Vector|MakeVector (* (Variables|GenerateMap|Getx) (Variables|GenerateMap|GetDistance)) (* (Variables|GenerateMap|Gety) (Variables|GenerateMap|GetDistance)) (Variables|Default|GetElevation)))
      (Components|StaticMesh|SetStaticMesh _ground (Variables|Meshes|GetGroundMesh))
      (bind _returnvalue_3 (Components|InstancedStaticMesh|AddInstance _ground (Math|Transform|MakeTransform (Math|Vector|MakeVector (* (Variables|GenerateMap|Getx) (Variables|GenerateMap|GetDistance)) (* (Variables|GenerateMap|Gety) (Variables|GenerateMap|GetDistance)) (Variables|Default|GetElevation)) "0, 0, 0" "1.000000,1.000000,1.000000") false))
      (Variables|Default|SetIndex _returnvalue_3)
      (Components|InstancedStaticMesh|SetCustomDataValue (Variables|Default|GetGround) (Variables|Default|GetIndex) 0 (Variables|Default|GetElevation) false)
      (Components|InstancedStaticMesh|SetCustomDataValue (Variables|Default|GetGround) (Variables|Default|GetIndex) 1 (Variables|MapConfiguration|GetSandHeight) false)
      (bind _returnvalue_4 (Utilities|Array|Add (Variables|GenerateMap|GetGridCell) (Variables|GenerateMap|GetGridVector)))
      (GenerateMap|AddTrees _returnvalue_4 (Variables|MapConfiguration|GetTreeDensity) (Variables|GenerateMap|GetTree%20Height%20Limit%20Water) 169.0)
      (GenerateMap|AddRocks _returnvalue_4 (Variables|MapConfiguration|GetRockDensity))
      (GenerateMap|AddWater))))

(fn AddTrees
  (params (GridIndex%20 :type Integer) (TreeDensity :type Float%20%28double-precision%29) (HeightLimitWater :type Float%20%28double-precision%29) (HeightLimitSnow :type Float%20%28double-precision%29))
  (bind _returnvalue (Math|Random|RandomFloatinRange 1.5 2.4))
  (bind _tree (Variables|Default|GetTree))
  (bind _gridcell (Variables|GenerateMap|GetGridCell))
  (bind _ground (Variables|Default|GetGround))
  (bind _returnvalue_2 (Transformation|GetWorldScale _ground))
  (bind _output (Utilities|Array|Get(acopy) _gridcell GridIndex%20))
  (if (<= (Math|Random|RandomIntegerinRange 0 100) (* TreeDensity 1e+02))
    (Components|StaticMesh|SetStaticMesh _tree (Variables|Meshes|GetTreeMesh))
    (if (and (> (.z _output) HeightLimitWater) (< (.z _output) HeightLimitSnow))
      (bind _returnvalue_3 (Components|InstancedStaticMesh|AddInstance _tree (Math|Transform|MakeTransform (Math|Vector|MakeVector (Math|Random|RandomFloatinRange (.x _output) (+ (.x _output) 1e+02)) (Math|Random|RandomFloatinRange (.y _output) (+ (.y _output) 5e+01)) (+ (* (.z _output) (.z _returnvalue_2)) (* (.z _returnvalue_2) 1e+02))) (Math|Rotator|MakeRotator 0.0 0.0 (Math|Random|RandomFloatinRange 0.0 3.6e+02)) (Math|Vector|MakeVector _returnvalue _returnvalue _returnvalue)) false))
      (Utilities|Array|AddUnique (Variables|Default|GetIndexTrees) _returnvalue_3))))

(fn RandomizeMap
  (bind _output_get (Variables|MapConfiguration|SetSize (Math|Random|RandomIntegerinRange 50 100)))
  (bind _output_get_2 (Variables|MapConfiguration|SetSeed (Math|Random|RandomIntegerinRange -100000000 100000000)))
  (bind _output_get_3 (Variables|MapConfiguration|SetFrequency (Math|Random|RandomFloatinRange 0.01 0.0515))))

(fn AddEnvironments)

(fn AddRocks
  (params (GridIndex :type Integer) (RockDensity :type Float%20%28double-precision%29))
  (bind _returnvalue (Math|Random|RandomFloatinRange 0.2 0.65))
  (bind _rock (Variables|Default|GetRock))
  (bind _gridcell (Variables|GenerateMap|GetGridCell))
  (bind _ground (Variables|Default|GetGround))
  (bind _returnvalue_2 (Transformation|GetWorldScale _ground))
  (bind _output (Utilities|Array|Get(acopy) _gridcell GridIndex))
  (if (<= (Math|Random|RandomIntegerinRange 0 100) (* RockDensity 1e+02))
    (Components|StaticMesh|SetStaticMesh _rock (Variables|Meshes|GetRockMesh))
    (bind _returnvalue_3 (Components|InstancedStaticMesh|AddInstance _rock (Math|Transform|MakeTransform (Math|Vector|MakeVector (Math|Random|RandomFloatinRange (.x _output) (+ (.x _output) 5e+01)) (Math|Random|RandomFloatinRange (.y _output) (+ (.y _output) 5e+01)) (+ (* (.z _output) (.z _returnvalue_2)) (* (.z _returnvalue_2) 1e+02))) (Math|Rotator|MakeRotator 0.0 0.0 (Math|Random|RandomFloatinRange 0.0 3.6e+02)) (Math|Vector|MakeVector _returnvalue _returnvalue _returnvalue)) false))
    (Utilities|Array|AddUnique (Variables|Default|GetIndexRocks) _returnvalue_3)))

(fn FillWater)

(fn GetInstancedStaticMeshTreeComponent
  (bind _indextrees (Variables|Default|GetIndexTrees))
  (bind _outitem (Utilities|Array|Random _indextrees))
  (return (.OutInstanceTransform (Components|InstancedStaticMesh|GetInstanceTransform (Variables|Default|GetTree) _outitem false)) _outitem))

(fn DestroyInstancedStaticMeshTreeComponent
  (params (Index :type Integer))
  (Utilities|Array|RemoveIndex (Variables|Default|GetIndexTrees) Index)
  (Class|InstancedStaticMeshComponent|RemoveInstance (Variables|Default|GetTree) Index))

(fn AddWater
  (bind _gridvector (Variables|GenerateMap|GetGridVector))
  (bind (_x _y) (Math|Vector|BreakVector _gridvector))
  (if (and (Variables|MapConfiguration|GetGeneratedWater?) (<= (Variables|Default|GetElevation) (Variables|MapConfiguration|GetHeightWater)))
    (Components|InstancedStaticMesh|AddInstance (Variables|Default|GetWater) (Math|Transform|MakeTransform (Math|Vector|MakeVector _x _y (Variables|MapConfiguration|GetHeightWater)) "0, 0, 0" "1.000000,1.000000,0.000000") false)))